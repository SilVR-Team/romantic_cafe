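; Café customer NPC that walks to the counter, voices a drink order, waits, then collects it and leaves.
; SetNPC stores menu, cream and ice; ActionStart rings and moves it over, then greeting, menu and option clips play sequenced by clip-length delays.
; SetOrder sends the order to BP_OrderManager before a looping wait animation.
; TakeOut notifies the manager, says goodbye, returns to BP_AI_Spawner, clears its customer flag and destroys itself.
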(event `self.ReceiveTick`
  (params (DeltaSeconds :type "Float (single-precision)"))
  (bind (_returnvalue_roll _returnvalue_pitch _returnvalue_yaw) (`KismetMathLibrary.BreakRotator` (`KismetMathLibrary.FindLookAtRotation` (`self.K2_GetActorLocation`) (`self.K2_GetActorLocation` (`GameplayStatics.GetPlayerPawn` 0)))))
  ;[1 1 1] Tick Event - 플레이어 바라보기
  (if (`self.isorder?`)
    (`self.K2_SetActorRotation` (`KismetMathLibrary.MakeRotator` 0.0 0.0 _returnvalue_yaw))))

(event `Set NPC`
  (params (Menu :type "/Game/CoreVR/Blueprints/Tools_Liquid/E_Liquid Enum" :default "NewEnumerator5") (`Cream?` :type Boolean) (`Ice?` :type Boolean))
  ;[1 1 1] 주문정보 받아오기
  (set `self.Menu` Menu)
  (set `self.Cream?` `Cream?`)
  (set `self.Ice?` `Ice?`)
  (`KismetSystemLibrary.Delay` 2.0)
  (`self.ActionStart`))

(event `ActionStart`
  (bind (_returnvalue_roll _returnvalue_pitch _returnvalue_yaw) (`KismetMathLibrary.BreakRotator` (`KismetMathLibrary.FindLookAtRotation` (`self.K2_GetActorLocation`) (`self.K2_GetActorLocation` (`GameplayStatics.GetPlayerPawn` 0)))))
  ;[1 0 0] NPC 활동 시작
  (`GameplayStatics.PlaySoundAtLocation` "/Game/CoreVR/Audio/Ring_Cue.Ring_Cue" (`self.K2_GetActorLocation`) (struct) 1.0 1.0 0.0 null null null null)
  (`AITask_MoveTo.AIMoveTo` (`AIBlueprintHelperLibrary.GetAIController` self) (-110.0 -80.0 108.0) null
    (:`OnMoveFinished`
      (set `self.isorder?` true)
      (`self.K2_SetActorRotation` (`KismetMathLibrary.MakeRotator` 0.0 0.0 _returnvalue_yaw))
      (`|PlayMontage` (`self.Mesh`) (`self.OrderAnim`)
        (:`then`
          (`self.oreder`))))))

(event `GoToHome`
  ;[1 0 0] NPC 퇴장
  (`self.StopAnimMontage` null)
  (bind _returnvalue (`GameplayStatics.GetActorOfClass` "/Game/CoreVR/Blueprints/NPC/BP_AI_Spawner.BP_AI_Spawner_C"))
  (`AITask_MoveTo.AIMoveTo` (`AIBlueprintHelperLibrary.GetAIController` self) (`self.K2_GetActorLocation` _returnvalue) null
    (:`OnMoveFinished`
      (set `/Game/CoreVR/Blueprints/NPC/BP_AI_Spawner.is customer exist` false _returnvalue)
      (`KismetSystemLibrary.Delay` 0.2)
      (`self.K2_DestroyActor`))))

(event `SetOrder`
  ;[1 1 1] BP_OrderManager에 메뉴 입력
  (bind _returnvalue (`GameplayStatics.GetActorOfClass` "/Game/CoreVR/Blueprints/Tools_Game/BP_OrderManager.BP_OrderManager_C"))
  (`/Game/CoreVR/Blueprints/Tools_Game/BP_OrderManager.Set Info` _returnvalue (`self.Menu`) (`self.Cream?`) (`self.Ice?`))
  (set `self.isorder?` false)
  (`self.GoToWaiting`))

(event `GoToWaiting`
  ;[1 0 0] NPC 대기 애니메이션 루프
  (`self.StopAnimMontage` null)
  (`AITask_MoveTo.AIMoveTo` (`AIBlueprintHelperLibrary.GetAIController` self) (`self.Waiting Location`) null
    (:`OnMoveFinished`
      (`self.K2_SetActorRotation` (struct))
      (`|PlayMontage` (`self.Mesh`) (`self.WaitAnim`) 1.0 0.0 "hi" :!label _label
        (:`OnCompleted`
          (goto _label))))))

(event `TakeOut`
  (bind (_returnvalue_roll _returnvalue_pitch _returnvalue_yaw) (`KismetMathLibrary.BreakRotator` (`KismetMathLibrary.FindLookAtRotation` (`self.K2_GetActorLocation`) (`self.K2_GetActorLocation` (`GameplayStatics.GetPlayerPawn` 0)))))
  ;[1 0 0] 제작이 완료된 메뉴를 회수 - BP_OrderManager
  (`self.StopAnimMontage` null)
  (`AITask_MoveTo.AIMoveTo` (`AIBlueprintHelperLibrary.GetAIController` self) (-110.0 -80.0 108.0) null
    (:`OnMoveFinished`
      (set `self.isorder?` true)
      (bind _returnvalue (`GameplayStatics.GetActorOfClass` "/Game/CoreVR/Blueprints/Tools_Game/BP_OrderManager.BP_OrderManager_C"))
      (`/Game/CoreVR/Blueprints/Tools_Game/BP_OrderManager.NPC Takeout` _returnvalue)
      (`self.K2_SetActorRotation` (`KismetMathLibrary.MakeRotator` 0.0 0.0 _returnvalue_yaw))
      (`self.PlayAnimMontage` (`self.OrderAnim`))
      (bind _output_get (set `self.ByeSound` (`KismetArrayLibrary.Array_Random` (`.Goodbyes_16_746DE9F54066B526B0CB6AB10EBACA9D` (break `/Game/CoreVR/Blueprints/NPC/ST_NPC` (`self.ST SoundCue`))))))
      (`GameplayStatics.PlaySoundAtLocation` _output_get (0.0 0.0 0.0) (struct) 1.0 1.0 0.0 null null null null)
      (`KismetSystemLibrary.Delay` (`SoundBase.Duration` _output_get))
      (set `self.isorder?` false)
      (`self.GoToHome`))))

(event `oreder`
  (bind ((`Ice_48_9B226BBE4919EDB613B9E0861D659C52` _ice) (`WhippingCream_50_31622D914A28DF3A2F306098245CD55A` _whippingcream) (`IceWhippingCream_53_370286764C72CB0F7FBD1AA1D2EB6339` _icewhippingcream)) (break `/Game/CoreVR/Blueprints/NPC/ST_NPC` (`self.ST SoundCue`)))
  (bind ((`Ice_48_9B226BBE4919EDB613B9E0861D659C52` _ice_2) (`WhippingCream_50_31622D914A28DF3A2F306098245CD55A` _whippingcream_2) (`IceWhippingCream_53_370286764C72CB0F7FBD1AA1D2EB6339` _icewhippingcream_2) (`Espresso_18_05F675B44D366E3678A387AFF06680A7` _espresso) (`ChocolateLatte_27_1A26B4D94A389A32A4B8CE854B7B7A89` _chocolatelatte) (`HazelnutCaffèMocha_28_B9E0417B479BDB0E5037EE8EBABF36E7` `_hazelnutcaffèmocha`) (`HazelnutLatte_116_263287B440554B46913F15A78B19095A` _hazelnutlatte) (`CaramelMacchiato_30_7DDFA80F4F331EE6169F73925E5D3CC2` _caramelmacchiato) (`HazelnutAmericano_31_D84531D544CC9F04D8725095F320FB88` _hazelnutamericano) (`VanillaAmericano_32_4DD247D24C80224CAA1C0280EB5322A9` _vanillaamericano) (`CaffèEinspänner_33_A74EE3FB40BC937B4E3A25BFD627F8DE` `_caffèeinspänner`) (`Americano_34_F8AE83024810B861982283A86C2810D6` _americano) (`ChocolateVanillaLatte_39_C0597E50441E4294832FAB92122D3DD7` _chocolatevanillalatte) (`VanillaLatte_40_60AB7F29433C63D049CBEB89B6668C5F` _vanillalatte) (`CaffèMocha_41_1FA72C3A47299202F598659E12D69A77` `_caffèmocha`) (`Mochaccino_42_B00D582446BC1C09A4EABF9A3A8AAF62` _mochaccino) (`Cappuccino_44_C863D1134140D96CCBB039B4FB095CE7` _cappuccino) (`Cortado_46_BACBD43B442E4FE0562F4B9D6321C3A5` _cortado)) (break `/Game/CoreVR/Blueprints/NPC/ST_NPC` (`self.ST SoundCue`)))
  ;[1 0.3185 0] 메뉴 주문 & 음성재생
  (bind _output_get (set `self.HelloSound` (`KismetArrayLibrary.Array_Random` (`.Greetings_12_9AB37A5F4FF335049CB148A4ADB53A03` (break `/Game/CoreVR/Blueprints/NPC/ST_NPC` (`self.ST SoundCue`))))))
  (`GameplayStatics.PlaySoundAtLocation` _output_get (0.0 0.0 0.0) (struct) 1.0 1.0 0.0 null null null null)
  (`KismetSystemLibrary.Delay` (+ (`SoundBase.Duration` _output_get) 0.6))
  (switch `/Game/CoreVR/Blueprints/Tools_Liquid/E_Liquid` (`self.Menu`)
    (:`NewEnumerator8`
      (`GameplayStatics.PlaySoundAtLocation` _espresso (0.0 0.0 0.0) (struct) 1.0 1.0 0.0 null null null null)
      (`KismetSystemLibrary.Delay` (`SoundBase.Duration` _espresso)))
    (:`NewEnumerator13`
      (`GameplayStatics.PlaySoundAtLocation` _chocolatelatte (0.0 0.0 0.0) (struct) 1.0 1.0 0.0 null null null null)
      (`KismetSystemLibrary.Delay` (`SoundBase.Duration` _chocolatelatte)))
    (:`NewEnumerator29`
      (`GameplayStatics.PlaySoundAtLocation` `_hazelnutcaffèmocha` (0.0 0.0 0.0) (struct) 1.0 1.0 0.0 null null null null)
      (`KismetSystemLibrary.Delay` (`SoundBase.Duration` `_hazelnutcaffèmocha`)))
    (:`NewEnumerator14`
      (`GameplayStatics.PlaySoundAtLocation` _hazelnutlatte (0.0 0.0 0.0) (struct) 1.0 1.0 0.0 null null null null)
      (`KismetSystemLibrary.Delay` (`SoundBase.Duration` _hazelnutlatte)))
    (:`NewEnumerator15`
      (`GameplayStatics.PlaySoundAtLocation` _caramelmacchiato (0.0 0.0 0.0) (struct) 1.0 1.0 0.0 null null null null)
      (`KismetSystemLibrary.Delay` (`SoundBase.Duration` _caramelmacchiato)))
    (:`NewEnumerator16`
      (`GameplayStatics.PlaySoundAtLocation` _hazelnutamericano (0.0 0.0 0.0) (struct) 1.0 1.0 0.0 null null null null)
      (`KismetSystemLibrary.Delay` (`SoundBase.Duration` _hazelnutamericano)))
    (:`NewEnumerator17`
      (`GameplayStatics.PlaySoundAtLocation` _vanillaamericano (0.0 0.0 0.0) (struct) 1.0 1.0 0.0 null null null null)
      (`KismetSystemLibrary.Delay` (`SoundBase.Duration` _vanillaamericano)))
    (:`NewEnumerator18`
      (`GameplayStatics.PlaySoundAtLocation` `_caffèeinspänner` (0.0 0.0 0.0) (struct) 1.0 1.0 0.0 null null null null)
      (`KismetSystemLibrary.Delay` (`SoundBase.Duration` `_caffèeinspänner`)))
    (:`NewEnumerator19`
      (`GameplayStatics.PlaySoundAtLocation` _americano (0.0 0.0 0.0) (struct) 1.0 1.0 0.0 null null null null)
      (`KismetSystemLibrary.Delay` (`SoundBase.Duration` _americano)))
    (:`NewEnumerator20`
      (`GameplayStatics.PlaySoundAtLocation` _chocolatevanillalatte (0.0 0.0 0.0) (struct) 1.0 1.0 0.0 null null null null)
      (`KismetSystemLibrary.Delay` (`SoundBase.Duration` _chocolatevanillalatte)))
    (:`NewEnumerator24`
      (`GameplayStatics.PlaySoundAtLocation` _vanillalatte (0.0 0.0 0.0) (struct) 1.0 1.0 0.0 null null null null)
      (`KismetSystemLibrary.Delay` (`SoundBase.Duration` _vanillalatte)))
    (:`NewEnumerator25`
      (`GameplayStatics.PlaySoundAtLocation` `_caffèmocha` (0.0 0.0 0.0) (struct) 1.0 1.0 0.0 null null null null)
      (`KismetSystemLibrary.Delay` (`SoundBase.Duration` `_caffèmocha`)))
    (:`NewEnumerator30`
      (`GameplayStatics.PlaySoundAtLocation` _mochaccino (0.0 0.0 0.0) (struct) 1.0 1.0 0.0 null null null null)
      (`KismetSystemLibrary.Delay` (`SoundBase.Duration` _mochaccino)))
    (:`NewEnumerator26`
      (`GameplayStatics.PlaySoundAtLocation` _cappuccino (0.0 0.0 0.0) (struct) 1.0 1.0 0.0 null null null null)
      (`KismetSystemLibrary.Delay` (`SoundBase.Duration` _cappuccino)))
    (:`NewEnumerator27`
      (`GameplayStatics.PlaySoundAtLocation` _cortado (0.0 0.0 0.0) (struct) 1.0 1.0 0.0 null null null null)
      (`KismetSystemLibrary.Delay` (`SoundBase.Duration` _cortado))))
  (if (`self.Cream?`)
    (if (`self.Ice?`)
      (`GameplayStatics.PlaySoundAtLocation` _icewhippingcream (0.0 0.0 0.0) (struct) 1.0 1.0 0.0 null null null null)
      (`KismetSystemLibrary.Delay` (`SoundBase.Duration` _icewhippingcream))
      (else
        (`GameplayStatics.PlaySoundAtLocation` _whippingcream (0.0 0.0 0.0) (struct) 1.0 1.0 0.0 null null null null)
        (`KismetSystemLibrary.Delay` (`SoundBase.Duration` _whippingcream))))
    (elif (`self.Ice?`)
      (`GameplayStatics.PlaySoundAtLocation` _ice (0.0 0.0 0.0) (struct) 1.0 1.0 0.0 null null null null)
      (`KismetSystemLibrary.Delay` (`SoundBase.Duration` _ice))))
  (`self.SetOrder`))

(fn `UserConstructionScript`)