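; BP_AI_Spawner spawns café customer NPCs and assigns each a drink order.
; While switched on, a looping timer spawns a random pawn class if no customer exists.
; Orders combine a random enabled menu item from the PlayerInfo save with weighted cream and ice rolls, converting Americano with cream to Einspänner, then go to BP_NPC via SetNPC.
; TutorialSpawn bypasses this with a fixed Americano order without cream or ice.
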(event `Spawner ON`
  ;[1 1 1] Spawner 작동 시작
  (set `self.switch on` true)
  (bind _returnvalue (`KismetSystemLibrary.K2_SetTimerDelegate` (delegate `spawn_ai`) (`self.SpawnLoopTime`) true))
  (set `self.Timer` _returnvalue)
  (`KismetSystemLibrary.Delay` 30.0)
  (if (`self.switch on`)
    (`self.spawn_ai`)))

(event `Spawner OFF`
  ;[1 1 1] Spawner 작동 중지
  (`KismetSystemLibrary.K2_ClearAndInvalidateTimerHandle` (`self.Timer`))
  (set `self.switch on` false))

(event `spawn_ai`
  (bind _trueindex (`self.TrueIndex`))
  ;[1 1 1] NPC 스폰 & 메뉴 선정
  (if (`self.switch on`)
    (if (not (`self.is customer exist`))
      (bind _returnvalue (`GameplayStatics.DoesSaveGameExist` "PlayerInfo"))
      (if _returnvalue
        (bind _returnvalue_2 (`GameplayStatics.LoadGameFromSlot` "PlayerInfo"))
        (bind _assv_player_info (cast `/Game/CoreVR/Blueprints/Player/SV_PlayerInfo` _returnvalue_2))
        (`KismetArrayLibrary.Array_Clear` (`self.TrueIndex`))
        (bind _output_get (set `self.Menu` (`/Game/CoreVR/Blueprints/Player/SV_PlayerInfo.Menu` _assv_player_info)))
        (bind _values (`BlueprintMapLibrary.Map_Values` _output_get))
        (for (_array_element _array_index) _values
          (if _array_element
            (`KismetArrayLibrary.Array_AddUnique` (`self.TrueIndex`) _array_index)))
        ;;[1 1 1] NPC 스폰
        (if (not (`KismetArrayLibrary.Array_IsEmpty` (`self.TrueIndex`)))
          (set `self.is customer exist` true)
          (bind _returnvalue_3 (`AIBlueprintHelperLibrary.SpawnAIFromClass` (`KismetArrayLibrary.Array_Random` (`self.Pawn Class`)) null (`self.K2_GetActorLocation`) (struct) false null))
          ;;[1 1 1] 메뉴 랜덤 선정
          (bind _asbp_npc (cast `/Game/CoreVR/Blueprints/NPC/BP_NPC` _returnvalue_3))
          (if true
            (bind _keys (`BlueprintMapLibrary.Map_Keys` (`self.Menu`)))
            (set `self.Now Menu` (`|GetArrayItem` _keys (`KismetArrayLibrary.Array_Random` (`self.TrueIndex`))))
            (else
              (bind _keys_2 (`BlueprintMapLibrary.Map_Keys` (`self.Menu`)))
              (set `self.Now Menu` (`KismetArrayLibrary.Array_Random` _keys_2))))
          (set `self.Now Cream` (`KismetMathLibrary.RandomBoolWithWeight` (`self.CreamPercent`)))
          (set `self.Now Ice` (`KismetMathLibrary.RandomBoolWithWeight` (`self.IcePercent`)))
          ;;[1 1 1] 아인슈페너 예외처리 (아메리카노 + 휘핑크림 = 아인슈페너)
          (bind _keys_3 (`BlueprintMapLibrary.Map_Keys` (`self.Menu`)))
          (if (and (`|EnumEquality` (`|GetArrayItem` _keys_3 (`|GetArrayItem` _trueindex)) "NewEnumerator19") (== (`KismetArrayLibrary.Array_Length` _trueindex) 1))
            (set `self.Now Cream` false))
          (if (and (`|EnumEquality` (`self.Now Menu`) "NewEnumerator19") (`self.Now Cream`))
            (set `self.Now Menu` "NewEnumerator18")
            (set `self.Now Cream` false))
          (if (and (`|EnumEquality` (`self.Now Menu`) "NewEnumerator18") (`self.Now Cream`))
            (set `self.Now Cream` false))
          (`/Game/CoreVR/Blueprints/NPC/BP_NPC.Set NPC` _asbp_npc (`self.Now Menu`) (`self.Now Cream`) (`self.Now Ice`))
          (set `self.Now NPC` _asbp_npc))))))

(event `Tutorial Spawn`
  ;[1 1 1] 튜토리얼 메뉴 제공
  (bind _returnvalue (`AIBlueprintHelperLibrary.SpawnAIFromClass` (`KismetArrayLibrary.Array_Random` (`self.Pawn Class`)) null (`self.K2_GetActorLocation`) (struct) false null))
  (bind _asbp_npc (cast `/Game/CoreVR/Blueprints/NPC/BP_NPC` _returnvalue))
  (set `self.Now Menu` "NewEnumerator19")
  (set `self.Now Cream` false)
  (set `self.Now Ice` false)
  (`/Game/CoreVR/Blueprints/NPC/BP_NPC.Set NPC` _asbp_npc (`self.Now Menu`) (`self.Now Cream`) (`self.Now Ice`))
  (set `self.Now NPC` _asbp_npc)
  (set `self.is customer exist` true))

(fn `UserConstructionScript`)