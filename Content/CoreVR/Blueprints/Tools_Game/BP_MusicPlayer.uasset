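; BP_MusicPlayer is a VR music player with touch buttons for play/pause, previous/next track and volume.
; Button collision overlaps step through a wrapping playlist, fade 2D sounds in and out, and update the UI_MusicInfo widget.
; Presses play a click, tint buttons red through dynamic materials, and send haptics to the hand identified by component tag.
; Enable flags and delays debounce track and play/pause presses, while volume changes in small clamped steps.
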(event `self.ReceiveBeginPlay`
  ;[1 0.3185 0] Dynamic Material 생성 및 적용
  (`|ExecutionSequence`
    (:`then_0`
      (bind _asui_music_info (cast `/Game/CoreVR/Blueprints/Widget/UI_MusicInfo` (`WidgetComponent.GetWidget` (`self.Widget`))))
      (set `self.As UI Music Info` _asui_music_info)
      (bind _returnvalue (`PrimitiveComponent.CreateDynamicMaterialInstance` (`self.NextButton`) 0 "/Game/Asset/CustomMesh/Material/M_Button.M_Button" "None"))
      (bind _output_get (set `self.MI_Next_Button` _returnvalue))
      (`MaterialInstanceDynamic.SetVectorParameterValue` _output_get "Color" (struct :`R` 1.0 :`G` 1.0 :`B` 1.0 :`A` 1.0))
      ;[1 0 0.8515] UI 기본값 적용
      (set `/Game/CoreVR/Blueprints/Widget/UI_MusicInfo.MusicVolume` (`KismetMathLibrary.FTrunc` (* (`self.Volume Multiplier`) 100.0)) (`self.As UI Music Info`))
      (set `/Game/CoreVR/Blueprints/Widget/UI_MusicInfo.MusicName` (`KismetTextLibrary.Conv_StringToText` (`|GetArrayItem` (`self.PlayListName`) (`self.PlayIndex`))) (`self.As UI Music Info`))
      (set `/Game/CoreVR/Blueprints/Widget/UI_MusicInfo.Play?` (`self.Play?`) (`self.As UI Music Info`))
      ;[1 1 1] 초기값 설정
      (bind _returnvalue_2 (`GameplayStatics.CreateSound2D` (`|GetArrayItem` (`self.PlayList`) (`self.PlayIndex`)) (`self.Volume Multiplier`) 1.0 0.0 null))
      (set `self.NowPlayingBGM` _returnvalue_2))
    (:`then_1`
      (bind _returnvalue_3 (`PrimitiveComponent.CreateDynamicMaterialInstance` (`self.PrevButton`) 0 "/Game/Asset/CustomMesh/Material/M_Button.M_Button" "None"))
      (bind _output_get_2 (set `self.MI_Prev_Button` _returnvalue_3))
      (`MaterialInstanceDynamic.SetVectorParameterValue` _output_get_2 "Color" (struct :`R` 1.0 :`G` 1.0 :`B` 1.0 :`A` 1.0)))
    (:`then_2`
      (bind _returnvalue_4 (`PrimitiveComponent.CreateDynamicMaterialInstance` (`self.SoundUPButton`) 0 "/Game/Asset/CustomMesh/Material/M_Button.M_Button" "None"))
      (bind _output_get_3 (set `self.MI_UP_Button` _returnvalue_4))
      (`MaterialInstanceDynamic.SetVectorParameterValue` _output_get_3 "Color" (struct :`R` 1.0 :`G` 1.0 :`B` 1.0 :`A` 1.0)))
    (:`then_3`
      (bind _returnvalue_5 (`PrimitiveComponent.CreateDynamicMaterialInstance` (`self.SoundDNButton`) 0 "/Game/Asset/CustomMesh/Material/M_Button.M_Button" "None"))
      (bind _output_get_4 (set `self.MI_DN_Button` _returnvalue_5))
      (`MaterialInstanceDynamic.SetVectorParameterValue` _output_get_4 "Color" (struct :`R` 1.0 :`G` 1.0 :`B` 1.0 :`A` 1.0)))
    (:`then_4`
      (bind _returnvalue_6 (`PrimitiveComponent.CreateDynamicMaterialInstance` (`self.PlayButton`) 0 "/Game/Asset/CustomMesh/Material/M_Button.M_Button" "None"))
      (bind _output_get_5 (set `self.MI_Play_Button` _returnvalue_6))
      (`MaterialInstanceDynamic.SetVectorParameterValue` _output_get_5 "Color" (struct :`R` 1.0 :`G` 1.0 :`B` 1.0 :`A` 1.0)))))

(event `self.NextCollision.OnComponentBeginOverlap`
  (params (OverlappedComponent :type "PrimitiveComponent Object Reference") (OtherActor :type "Actor Object Reference") (OtherComp :type "PrimitiveComponent Object Reference") (OtherBodyIndex :type Integer) (bFromSweep :type Boolean) (SweepResult :type "HitResult Structure (by ref)"))
  ;[1 0.3185 0] Haptic & Effect
  (if (`self.Enable?`)
    (`self.Haptic` OtherComp)
    (`|ExecutionSequence`
      (:`then_0`
        (set `self.Enable?` false)
        (`GameplayStatics.PlaySoundAtLocation` "/Game/CoreVR/Audio/Click_Cue.Click_Cue" (`self.K2_GetActorLocation`) (struct) 1.0 1.0 0.0 null null null null)
        ;[1 0 0] Next Button
        (bind _result (`/Engine/EditorBlueprintResources/StandardMacros.IncrementInt` (`self.PlayIndex`))
          (:`  `
            (if (> _result (`KismetArrayLibrary.Array_LastIndex` (`self.PlayList`)))
              (set `self.PlayIndex` 0))
            (if (`self.Play?`)
              (`AudioComponent.FadeOut` (`self.NowPlayingBGM`) 0.5 0.0 "Linear")
              (`KismetSystemLibrary.Delay` 1.0)
              (bind _returnvalue (`GameplayStatics.CreateSound2D` (`|GetArrayItem` (`self.PlayList`) (`self.PlayIndex`)) 1.0 1.0 0.0 null))
              (bind _output_get (set `self.NowPlayingBGM` _returnvalue))
              (`AudioComponent.FadeIn` _output_get 0.5 1.0 0.0 "Linear")
              (`AudioComponent.AdjustVolume` _output_get 0.0 (`self.Volume Multiplier`) "Linear")
              (else
                (bind _returnvalue_2 (`GameplayStatics.CreateSound2D` (`|GetArrayItem` (`self.PlayList`) (`self.PlayIndex`)) 1.0 1.0 0.0 null))
                (set `self.NowPlayingBGM` _returnvalue_2)))
            ;[1 0 0.8515] UI 적용
            (set `/Game/CoreVR/Blueprints/Widget/UI_MusicInfo.MusicName` (`KismetTextLibrary.Conv_StringToText` (`|GetArrayItem` (`self.PlayListName`) (`self.PlayIndex`))) (`self.As UI Music Info`) :!label _label)
            (set `self.Enable?` true)
            (`KismetSystemLibrary.Delay` 0.1)
            (`MaterialInstanceDynamic.SetVectorParameterValue` (`self.MI_Next_Button`) "Color" (struct :`R` 1.0 :`G` 1.0 :`B` 1.0 :`A` 1.0))
            (`MaterialInstanceDynamic.SetVectorParameterValue` (`self.MI_Prev_Button`) "Color" (struct :`R` 1.0 :`G` 1.0 :`B` 1.0 :`A` 1.0)))))
      (:`then_1`
        (`MaterialInstanceDynamic.SetVectorParameterValue` (`self.MI_Next_Button`) "Color" (struct :`R` 1.0 :`A` 1.0))))))

(event `self.PrevCollision.OnComponentBeginOverlap`
  (params (OverlappedComponent :type "PrimitiveComponent Object Reference") (OtherActor :type "Actor Object Reference") (OtherComp :type "PrimitiveComponent Object Reference") (OtherBodyIndex :type Integer) (bFromSweep :type Boolean) (SweepResult :type "HitResult Structure (by ref)"))
  ;[1 0.3185 0] Haptic & Effect
  (if (`self.Enable?`)
    (`self.Haptic` OtherComp)
    (`|ExecutionSequence`
      (:`then_0`
        (set `self.Enable?` false)
        (`GameplayStatics.PlaySoundAtLocation` "/Game/CoreVR/Audio/Click_Cue.Click_Cue" (`self.K2_GetActorLocation`) (struct) 1.0 1.0 0.0 null null null null)
        ;[1 0 0] Previous Button
        (bind _result (`/Engine/EditorBlueprintResources/StandardMacros.DecrementInt` (`self.PlayIndex`))
          (:`  `
            (if (< _result 0)
              (set `self.PlayIndex` (`KismetArrayLibrary.Array_LastIndex` (`self.PlayList`))))
            (if (`self.Play?`)
              (`AudioComponent.FadeOut` (`self.NowPlayingBGM`) 0.5 0.0 "Linear")
              (`KismetSystemLibrary.Delay` 1.0)
              (bind _returnvalue (`GameplayStatics.CreateSound2D` (`|GetArrayItem` (`self.PlayList`) (`self.PlayIndex`)) 1.0 1.0 0.0 null))
              (bind _output_get (set `self.NowPlayingBGM` _returnvalue))
              (`AudioComponent.FadeIn` _output_get 0.5 1.0 0.0 "Linear")
              (`AudioComponent.AdjustVolume` _output_get 0.0 (`self.Volume Multiplier`) "Linear")
              (goto _label)
              (else
                (bind _returnvalue_2 (`GameplayStatics.CreateSound2D` (`|GetArrayItem` (`self.PlayList`) (`self.PlayIndex`)) 1.0 1.0 0.0 null))
                (set `self.NowPlayingBGM` _returnvalue_2)
                (goto _label))))))
      (:`then_1`
        (`MaterialInstanceDynamic.SetVectorParameterValue` (`self.MI_Prev_Button`) "Color" (struct :`R` 1.0 :`A` 1.0))))))

(event `self.PlayCollision.OnComponentBeginOverlap`
  (params (OverlappedComponent :type "PrimitiveComponent Object Reference") (OtherActor :type "Actor Object Reference") (OtherComp :type "PrimitiveComponent Object Reference") (OtherBodyIndex :type Integer) (bFromSweep :type Boolean) (SweepResult :type "HitResult Structure (by ref)"))
  ;[1 0.3185 0] Haptic & Effect
  (if (`self.PlayEnable?`)
    (`self.Haptic` OtherComp)
    (set `self.PlayEnable?` false)
    (`GameplayStatics.PlaySoundAtLocation` "/Game/CoreVR/Audio/Click_Cue.Click_Cue" (`self.K2_GetActorLocation`) (struct) 1.0 1.0 0.0 null null null null)
    ;[1 0 0] Play/Pause Button
    (if (`self.Play?`)
      (`AudioComponent.FadeOut` (`self.NowPlayingBGM`) 0.5 0.0 "Linear")
      (set `self.Play?` false)
      (set `/Game/CoreVR/Blueprints/Widget/UI_MusicInfo.Play?` false (`self.As UI Music Info`))
      (else
        (bind _returnvalue (`GameplayStatics.CreateSound2D` (`|GetArrayItem` (`self.PlayList`) (`self.PlayIndex`)) 1.0 1.0 0.0 null))
        (bind _output_get (set `self.NowPlayingBGM` _returnvalue))
        (`AudioComponent.AdjustVolume` _output_get 0.0 (`self.Volume Multiplier`) "Linear")
        (`AudioComponent.FadeIn` _output_get 0.5 1.0 0.0 "Linear")
        (`AudioComponent.AdjustVolume` _output_get 0.0 (`self.Volume Multiplier`) "Linear")
        (set `self.Play?` true)
        (set `/Game/CoreVR/Blueprints/Widget/UI_MusicInfo.Play?` true (`self.As UI Music Info`))))
    (`KismetSystemLibrary.RetriggerableDelay` 1.0)
    (set `self.PlayEnable?` true)
    (if (`self.Play?`)
      (`MaterialInstanceDynamic.SetVectorParameterValue` (`self.MI_Play_Button`) "Color" (struct :`R` 1.0 :`A` 1.0))
      (else
        (`MaterialInstanceDynamic.SetVectorParameterValue` (`self.MI_Play_Button`) "Color" (struct :`R` 1.0 :`G` 1.0 :`B` 1.0 :`A` 1.0))))))

(event `self.SoundUPCollision.OnComponentBeginOverlap`
  (params (OverlappedComponent :type "PrimitiveComponent Object Reference") (OtherActor :type "Actor Object Reference") (OtherComp :type "PrimitiveComponent Object Reference") (OtherBodyIndex :type Integer) (bFromSweep :type Boolean) (SweepResult :type "HitResult Structure (by ref)"))
  ;[1 0.3185 0] Haptic & Effect
  (`self.Haptic` OtherComp)
  (`|ExecutionSequence`
    (:`then_0`
      (`GameplayStatics.PlaySoundAtLocation` "/Game/CoreVR/Audio/Click_Cue.Click_Cue" (`self.K2_GetActorLocation`) (struct) 1.0 1.0 0.0 null null null null)
      ;[1 0 0] Volume UP Button
      (set `self.Volume Multiplier` (`KismetMathLibrary.FClamp` (+ (`self.Volume Multiplier`) 0.02)))
      (bind _nowplayingbgm (`self.NowPlayingBGM`)
        (:`then`
          (`AudioComponent.AdjustVolume` _nowplayingbgm 0.0 (`self.Volume Multiplier`) "Linear"))
        (:`else`
          _))
      ;[1 0 0.8515] UI 적용
      (set `/Game/CoreVR/Blueprints/Widget/UI_MusicInfo.MusicVolume` (`KismetMathLibrary.FTrunc` (* (`self.Volume Multiplier`) 100.0)) (`self.As UI Music Info`) :!label _label_2))
    (:`then_1`
      (`MaterialInstanceDynamic.SetVectorParameterValue` (`self.MI_UP_Button`) "Color" (struct :`R` 1.0 :`A` 1.0))
      (`KismetSystemLibrary.RetriggerableDelay` 0.1)
      (`MaterialInstanceDynamic.SetVectorParameterValue` (`self.MI_UP_Button`) "Color" (struct :`R` 1.0 :`G` 1.0 :`B` 1.0 :`A` 1.0)))))

(event `self.SoundDNCollision.OnComponentBeginOverlap`
  (params (OverlappedComponent :type "PrimitiveComponent Object Reference") (OtherActor :type "Actor Object Reference") (OtherComp :type "PrimitiveComponent Object Reference") (OtherBodyIndex :type Integer) (bFromSweep :type Boolean) (SweepResult :type "HitResult Structure (by ref)"))
  ;[1 0.3185 0] Haptic & Effect
  (`self.Haptic` OtherComp)
  (`|ExecutionSequence`
    (:`then_0`
      (`GameplayStatics.PlaySoundAtLocation` "/Game/CoreVR/Audio/Click_Cue.Click_Cue" (`self.K2_GetActorLocation`) (struct) 1.0 1.0 0.0 null null null null)
      ;[1 0 0] Volume Down Button
      (set `self.Volume Multiplier` (`KismetMathLibrary.FClamp` (- (`self.Volume Multiplier`) 0.02)))
      (bind _nowplayingbgm (`self.NowPlayingBGM`)
        (:`then`
          (`AudioComponent.AdjustVolume` _nowplayingbgm 0.0 (`self.Volume Multiplier`) "Linear")
          (goto _label_2))
        (:`else`
          (goto _label_2))))
    (:`then_1`
      (`MaterialInstanceDynamic.SetVectorParameterValue` (`self.MI_DN_Button`) "Color" (struct :`R` 1.0 :`A` 1.0))
      (`KismetSystemLibrary.RetriggerableDelay` 0.1)
      (`MaterialInstanceDynamic.SetVectorParameterValue` (`self.MI_DN_Button`) "Color" (struct :`R` 1.0 :`G` 1.0 :`B` 1.0 :`A` 1.0)))))

(fn `UserConstructionScript`)