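; BP_TutorialPad is a VR pad with physical buttons that drive a UI_Tutorial widget showing tutorial and recipe pages.
; Collision overlaps page backward or forward, switch screens, or reset the pad's transform and first page, each playing a sound.
; Buttons flash via dynamic materials, with delay-based cooldowns debouncing all but the reset button.
; Haptic picks the controller from the overlapping component's Left/Right tag, using a different effect per hand.
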(event `self.ReceiveBeginPlay`
  ;[1 1 1] 초기 설정
  (bind _asui_tutorial (cast `/Game/CoreVR/Blueprints/Widget/UI_Tutorial` (`WidgetComponent.GetWidget` (`self.Widget`))))
  (bind _output_get (set `self.As UI Tutorial` _asui_tutorial))
  (`/Game/CoreVR/Blueprints/Widget/UI_Tutorial.Set First Page` _output_get (`self.Tutorial Page`) (`self.Recipe Page`) (`self.Recipe Screen First`))
  (set `self.Origin` (`SceneComponent.K2_GetComponentToWorld` (`self.Pad`)))
  ;[1 0.3185 0] 버튼 Dynamic Material 생성
  (bind _returnvalue (`PrimitiveComponent.CreateDynamicMaterialInstance` (`self.PreviousButton`) 0 "/Game/Asset/CustomMesh/Material/M_Button.M_Button" "None"))
  (set `self.MI_Prev_Button` _returnvalue)
  (`MaterialInstanceDynamic.SetVectorParameterValue` (`self.MI_Prev_Button`) "Color" (struct :`R` 1.0 :`A` 1.0))
  (bind _returnvalue_2 (`PrimitiveComponent.CreateDynamicMaterialInstance` (`self.NextButton`) 0 "/Game/Asset/CustomMesh/Material/M_Button.M_Button" "None"))
  (set `self.MI_Next_Button` _returnvalue_2)
  (`MaterialInstanceDynamic.SetVectorParameterValue` (`self.MI_Next_Button`) "Color" (struct :`R` 1.0 :`A` 1.0))
  (bind _returnvalue_3 (`PrimitiveComponent.CreateDynamicMaterialInstance` (`self.MidButton`) 0 "/Game/Asset/CustomMesh/Material/M_Button.M_Button" "None"))
  (set `self.MI_Mid_Button` _returnvalue_3)
  (`MaterialInstanceDynamic.SetVectorParameterValue` (`self.MI_Mid_Button`) "Color" (struct :`R` 1.0 :`A` 1.0))
  (bind _returnvalue_4 (`PrimitiveComponent.CreateDynamicMaterialInstance` (`self.InitializeButton`) 0 "/Game/Asset/CustomMesh/Material/M_Button.M_Button" "None"))
  (set `self.MI_Play_Button` _returnvalue_4)
  (`MaterialInstanceDynamic.SetVectorParameterValue` (`self.MI_Play_Button`) "Color" (struct :`R` 1.0 :`A` 1.0)))

(event `self.InitializeCollision.OnComponentBeginOverlap`
  (params (OverlappedComponent :type "PrimitiveComponent Object Reference") (OtherActor :type "Actor Object Reference") (OtherComp :type "PrimitiveComponent Object Reference") (OtherBodyIndex :type Integer) (bFromSweep :type Boolean) (SweepResult :type "HitResult Structure (by ref)"))
  ;[1 0 0] 화면/위치 초기화
  (`|ExecutionSequence`
    (:`then_0`
      (`SceneComponent.K2_SetWorldTransform` (`self.Pad`) (`self.Origin`) false false)
      (`self.Haptic` OtherComp)
      (`GameplayStatics.PlaySoundAtLocation` "/Game/CoreVR/Audio/Click_Cue.Click_Cue" (`self.K2_GetActorLocation`) (struct) 1.0 1.0 0.0 null null null null)
      (`/Game/CoreVR/Blueprints/Widget/UI_Tutorial.Set First Page` (`self.As UI Tutorial`) (`self.Tutorial Page`) (`self.Recipe Page`) (`self.Recipe Screen First`)))
    (:`then_1`
      (`MaterialInstanceDynamic.SetVectorParameterValue` (`self.MI_Play_Button`) "Color" (struct :`R` 1.0 :`G` 1.0 :`B` 1.0 :`A` 1.0))
      (`KismetSystemLibrary.Delay` 0.2)
      (`MaterialInstanceDynamic.SetVectorParameterValue` (`self.MI_Play_Button`) "Color" (struct :`R` 1.0 :`A` 1.0)))))

(event `self.PreviousCollision.OnComponentBeginOverlap`
  (params (OverlappedComponent :type "PrimitiveComponent Object Reference") (OtherActor :type "Actor Object Reference") (OtherComp :type "PrimitiveComponent Object Reference") (OtherBodyIndex :type Integer) (bFromSweep :type Boolean) (SweepResult :type "HitResult Structure (by ref)"))
  ;[1 0 0] Previous Button
  (if (not (`self.PrevCooldown`))
    (set `self.PrevCooldown` true)
    (`|ExecutionSequence`
      (:`then_0`
        ;[1 0.3185 0] Haptic & Sound &Effect
        (`self.Haptic` OtherComp)
        (`/Game/CoreVR/Blueprints/Widget/UI_Tutorial.Previous` (`self.As UI Tutorial`))
        (`GameplayStatics.PlaySoundAtLocation` "/Game/CoreVR/Audio/Page_Cue.Page_Cue" (`self.K2_GetActorLocation`) (struct) 1.0 1.0 0.0 null null null null))
      (:`then_1`
        (`MaterialInstanceDynamic.SetVectorParameterValue` (`self.MI_Prev_Button`) "Color" (struct :`R` 1.0 :`G` 1.0 :`B` 1.0 :`A` 1.0))
        (`KismetSystemLibrary.Delay` 0.2)
        (`MaterialInstanceDynamic.SetVectorParameterValue` (`self.MI_Prev_Button`) "Color" (struct :`R` 1.0 :`A` 1.0))
        (set `self.PrevCooldown` false)))))

(event `self.NextCollision.OnComponentBeginOverlap`
  (params (OverlappedComponent :type "PrimitiveComponent Object Reference") (OtherActor :type "Actor Object Reference") (OtherComp :type "PrimitiveComponent Object Reference") (OtherBodyIndex :type Integer) (bFromSweep :type Boolean) (SweepResult :type "HitResult Structure (by ref)"))
  ;[1 0 0] Next Button
  (if (not (`self.NextCooldown`))
    (set `self.NextCooldown` true)
    (`|ExecutionSequence`
      (:`then_0`
        ;[1 0.3185 0] Haptic & Sound &Effect
        (`self.Haptic` OtherComp)
        (`/Game/CoreVR/Blueprints/Widget/UI_Tutorial.Next` (`self.As UI Tutorial`))
        (`GameplayStatics.PlaySoundAtLocation` "/Game/CoreVR/Audio/Page_Cue.Page_Cue" (`self.K2_GetActorLocation`) (struct) 1.0 1.0 0.0 null null null null))
      (:`then_1`
        (`MaterialInstanceDynamic.SetVectorParameterValue` (`self.MI_Next_Button`) "Color" (struct :`R` 1.0 :`G` 1.0 :`B` 1.0 :`A` 1.0))
        (`KismetSystemLibrary.Delay` 0.2)
        (`MaterialInstanceDynamic.SetVectorParameterValue` (`self.MI_Next_Button`) "Color" (struct :`R` 1.0 :`A` 1.0))
        (set `self.NextCooldown` false)))))

(event `self.MidCollision.OnComponentBeginOverlap`
  (params (OverlappedComponent :type "PrimitiveComponent Object Reference") (OtherActor :type "Actor Object Reference") (OtherComp :type "PrimitiveComponent Object Reference") (OtherBodyIndex :type Integer) (bFromSweep :type Boolean) (SweepResult :type "HitResult Structure (by ref)"))
  ;[1 0 0] 화면전환
  (if (not (`self.MidCooldown`))
    (set `self.MidCooldown` true)
    (`|ExecutionSequence`
      (:`then_0`
        ;[1 0.3185 0] Haptic & Sound &Effect
        (`self.Haptic` OtherComp)
        (`/Game/CoreVR/Blueprints/Widget/UI_Tutorial.Change Home` (`self.As UI Tutorial`))
        (`GameplayStatics.PlaySoundAtLocation` "/Game/CoreVR/Audio/Page_Cue.Page_Cue" (`self.K2_GetActorLocation`) (struct) 1.0 1.0 0.0 null null null null))
      (:`then_1`
        (`MaterialInstanceDynamic.SetVectorParameterValue` (`self.MI_Mid_Button`) "Color" (struct :`R` 1.0 :`G` 1.0 :`B` 1.0 :`A` 1.0))
        (`KismetSystemLibrary.Delay` 0.2)
        (`MaterialInstanceDynamic.SetVectorParameterValue` (`self.MI_Mid_Button`) "Color" (struct :`R` 1.0 :`A` 1.0))
        (set `self.MidCooldown` false)))))

(fn `UserConstructionScript`)