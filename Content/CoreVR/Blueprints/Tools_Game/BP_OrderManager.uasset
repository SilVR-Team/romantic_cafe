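; VR drink-order station that shows the NPC's order on three menu widgets and checks the cup the player serves.
; A sphere detects the cup, and a call button compares its type, cream, temperature and amount to the order, then recalls the NPC or flags an error.
; A second button toggles the AI spawner, with cooldown and haptics.
; NPC takeout resets the cup and clears the saved tutorial flag.
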(event `self.ReceiveBeginPlay`
  ;[1 1 1] 초기 설정
  (bind _asui_menu_info (cast `/Game/CoreVR/Blueprints/Widget/UI_MenuInfo` (`WidgetComponent.GetWidget` (`self.Widget`))))
  (set `self.As UI Menu Info` _asui_menu_info)
  (bind _asui_menu_info_2 (cast `/Game/CoreVR/Blueprints/Widget/UI_MenuInfo` (`WidgetComponent.GetWidget` (`self.Widget2`))))
  (set `self.As UI Menu Info_1` _asui_menu_info_2)
  (bind _asui_menu_info_3 (cast `/Game/CoreVR/Blueprints/Widget/UI_MenuInfo` (`WidgetComponent.GetWidget` (`self.Widget1`))))
  (set `self.As UI Menu Info_0` _asui_menu_info_3)
  (bind _returnvalue (`PrimitiveComponent.CreateDynamicMaterialInstance` (`self.PrevButton`) 0 "/Game/Asset/CustomMesh/Material/M_Button.M_Button" "None"))
  (set `self.MI_Play_Button` _returnvalue)
  (`MaterialInstanceDynamic.SetVectorParameterValue` (`self.MI_Play_Button`) "Color" (struct :`R` 1.0 :`A` 1.0)))

(event `Tutorial Request`
  ;[1 1 1] 튜토리얼 요청
  (bind _returnvalue (`GameplayStatics.GetActorOfClass` "/Game/CoreVR/Blueprints/NPC/BP_AI_Spawner.BP_AI_Spawner_C"))
  (`/Game/CoreVR/Blueprints/NPC/BP_AI_Spawner.Tutorial Spawn` _returnvalue))

(event `Set Info`
  (params (Menu :type "/Game/CoreVR/Blueprints/Tools_Liquid/E_Liquid Enum" :default "NewEnumerator5") (`Cream?` :type Boolean) (`Ice?` :type Boolean))
  ;[1 1 1] NPC 음료 정보 받아오기
  (set `self.Menu` Menu)
  (set `self.Cream?` `Cream?`)
  (set `self.Ice?` `Ice?`)
  (`/Game/CoreVR/Blueprints/Widget/UI_MenuInfo.Set Info` (`self.As UI Menu Info`) (`self.Menu`) (`self.Cream?`) (`self.Ice?`))
  (`/Game/CoreVR/Blueprints/Widget/UI_MenuInfo.Set Info` (`self.As UI Menu Info_0`) (`self.Menu`) (`self.Cream?`) (`self.Ice?`))
  (`/Game/CoreVR/Blueprints/Widget/UI_MenuInfo.Set Info` (`self.As UI Menu Info_1`) (`self.Menu`) (`self.Cream?`) (`self.Ice?`)))

(event `NPC Takeout`
  ;[1 1 1] NPC가 음료를 가져감
  (bind _as_bp_test_cup (`self.As BP Test Cup`)
    (:`then`
      (set `self.Active` true)
      (`/Game/CoreVR/Blueprints/Tools_Liquid/BP_BaseCup.Reset Cup` _as_bp_test_cup)
      (set `self.CallCooldown` false)
      (bind _returnvalue (`GameplayStatics.LoadGameFromSlot` "PlayerInfo"))
      (bind _assv_player_info (cast `/Game/CoreVR/Blueprints/Player/SV_PlayerInfo` _returnvalue))
      (set `/Game/CoreVR/Blueprints/Player/SV_PlayerInfo.Tutorial?` false _assv_player_info)
      (`GameplayStatics.SaveGameToSlot` _assv_player_info "PlayerInfo"))
    (:`else`)))

(event `self.Sphere.OnComponentBeginOverlap`
  (params (OverlappedComponent :type "PrimitiveComponent Object Reference") (OtherActor :type "Actor Object Reference") (OtherComp :type "PrimitiveComponent Object Reference") (OtherBodyIndex :type Integer) (bFromSweep :type Boolean) (SweepResult :type "HitResult Structure (by ref)"))
  ;[1 0 0] 플레이어가 제공한 음료 정보 인식
  (if (`self.Active`)
    (bind _asbp_base_cup (cast `/Game/CoreVR/Blueprints/Tools_Liquid/BP_BaseCup` OtherActor))
    (bind _output_get (set `self.As BP Test Cup` _asbp_base_cup))
    (`SceneComponent.SetVisibility` (`self.TextRender2`) true false)
    (`SceneComponent.SetVisibility` (`self.TextRender1`) false false)
    (`PlayerController.PlayHapticEffect` (`GameplayStatics.GetPlayerController` 0) "/Game/CoreVR/Haptics/AttachHapticEffect.AttachHapticEffect" (`/Game/CoreVR/Blueprints/Component/BP_GrabComponent.GetHeldByHand` (`/Game/CoreVR/Blueprints/Tools_Liquid/BP_BaseCup.GrabComponent` _output_get)) 0.5 false)))

(event `self.Sphere.OnComponentEndOverlap`
  (params (OverlappedComponent :type "PrimitiveComponent Object Reference") (OtherActor :type "Actor Object Reference") (OtherComp :type "PrimitiveComponent Object Reference") (OtherBodyIndex :type Integer))
  ;[1 0 0] 플레이어가 제공한 음료 정보 인식
  (if (`self.Active`)
    (if (== OtherActor (`self.As BP Test Cup`))
      (set `self.As BP Test Cup` null)
      (`SceneComponent.SetVisibility` (`self.TextRender2`) false false)
      (`SceneComponent.SetVisibility` (`self.TextRender1`) true false))))

(event `self.PrevCollision.OnComponentBeginOverlap`
  (params (OverlappedComponent :type "PrimitiveComponent Object Reference") (OtherActor :type "Actor Object Reference") (OtherComp :type "PrimitiveComponent Object Reference") (OtherBodyIndex :type Integer) (bFromSweep :type Boolean) (SweepResult :type "HitResult Structure (by ref)"))
  (bind _canorder_ (`self.CanOrder?`))
  ;[1 0 0] NPC 소환 기능 활성화/비활성화
  (if (not (`self.OrderCooldown`))
    (`GameplayStatics.PlaySoundAtLocation` "/Game/CoreVR/Audio/Click_Cue.Click_Cue" (`self.K2_GetActorLocation`) (struct) 1.0 1.0 0.0 null null null null)
    (`self.Haptic` OtherComp)
    (`|ExecutionSequence`
      (:`then_0`
        (set `self.OrderCooldown` true)
        (if (`self.CanOrder?`)
          (set `self.CanOrder?` false)
          (else
            (set `self.CanOrder?` true)))
        ;;[1 0 0.8515] UI 적용
        (set `/Game/CoreVR/Blueprints/Widget/UI_MenuInfo.CanOrder?` _canorder_ (`self.As UI Menu Info`))
        (set `/Game/CoreVR/Blueprints/Widget/UI_MenuInfo.CanOrder?` _canorder_ (`self.As UI Menu Info_0`))
        (set `/Game/CoreVR/Blueprints/Widget/UI_MenuInfo.CanOrder?` _canorder_ (`self.As UI Menu Info_1`))
        (if (`self.CanOrder?`)
          (bind _returnvalue (`GameplayStatics.GetActorOfClass` "/Game/CoreVR/Blueprints/NPC/BP_AI_Spawner.BP_AI_Spawner_C"))
          (`/Game/CoreVR/Blueprints/NPC/BP_AI_Spawner.Spawner ON` _returnvalue)
          (else
            (bind _returnvalue_2 (`GameplayStatics.GetActorOfClass` "/Game/CoreVR/Blueprints/NPC/BP_AI_Spawner.BP_AI_Spawner_C"))
            (`/Game/CoreVR/Blueprints/NPC/BP_AI_Spawner.Spawner OFF` _returnvalue_2)))
        (`KismetSystemLibrary.Delay` 1.0)
        (set `self.OrderCooldown` false))
      (:`then_1`
        (`MaterialInstanceDynamic.SetVectorParameterValue` (`self.MI_Play_Button`) "Color" (struct :`R` 1.0 :`G` 1.0 :`B` 1.0 :`A` 1.0))
        (`KismetSystemLibrary.Delay` 1.0)
        (`MaterialInstanceDynamic.SetVectorParameterValue` (`self.MI_Play_Button`) "Color" (struct :`R` 1.0 :`A` 1.0))))))

(event `self.PlayCollision.OnComponentBeginOverlap`
  (params (OverlappedComponent :type "PrimitiveComponent Object Reference") (OtherActor :type "Actor Object Reference") (OtherComp :type "PrimitiveComponent Object Reference") (OtherBodyIndex :type Integer) (bFromSweep :type Boolean) (SweepResult :type "HitResult Structure (by ref)"))
  (bind _as_ui_menu_info (`self.As UI Menu Info`))
  ;[1 0 0] 플레이어가 제공한 음료가 주문한 메뉴와 일치하는 지 확인
  (if (not (`self.CallCooldown`))
    (`self.Haptic` OtherComp)
    (set `self.CallCooldown` true)
    (bind _as_bp_test_cup (`self.As BP Test Cup`)
      (:`then`
        (if (and (`|EnumEquality` (`self.Menu`) "NewEnumerator18") (`|EnumEquality` (`/Game/CoreVR/Blueprints/Tools_Liquid/BP_BaseCup.Now Type` _as_bp_test_cup) "NewEnumerator18") (== (`|EnumEquality` (`/Game/CoreVR/Blueprints/Tools_Liquid/BP_BaseCup.Temp` _as_bp_test_cup) "NewEnumerator14") (`self.Ice?`)))
          (if (>= (`/Game/CoreVR/Blueprints/Tools_Liquid/BP_BaseCup.Now Amount` _as_bp_test_cup) 80.0) :!label _label
            (set `self.Active` false)
            ;;[1 1 1] 일치하는 경우
            (`/Game/CoreVR/Blueprints/Widget/UI_MenuInfo.Equal` _as_ui_menu_info)
            (`/Game/CoreVR/Blueprints/Widget/UI_MenuInfo.Equal` (`self.As UI Menu Info_0`))
            (`/Game/CoreVR/Blueprints/Widget/UI_MenuInfo.Equal` (`self.As UI Menu Info_1`))
            (bind _returnvalue (`GameplayStatics.GetActorOfClass` "/Game/CoreVR/Blueprints/NPC/BP_AI_Spawner.BP_AI_Spawner_C"))
            (bind _now_npc (`/Game/CoreVR/Blueprints/NPC/BP_AI_Spawner.Now NPC` _returnvalue)
              (:`then`
                (`/Game/CoreVR/Blueprints/NPC/BP_NPC.comeback` _now_npc)
                (`GameplayStatics.PlaySoundAtLocation` "/Game/CoreVR/Audio/bell_Cue.bell_Cue" (0.0 0.0 0.0) (struct) 1.0 1.0 0.0 null null null null))
              (:`else`
                (set `self.Active` true)
                (`/Game/CoreVR/Blueprints/Tools_Liquid/BP_BaseCup.Reset Cup` _as_bp_test_cup)
                (`GameplayStatics.PlaySoundAtLocation` "/Game/CoreVR/Audio/bell_Cue.bell_Cue" (`self.K2_GetActorLocation`) (struct) 1.0 1.0 0.0 null null null null)
                (`KismetSystemLibrary.Delay` 0.5)
                (set `self.CallCooldown` false)))
            (else
              ;;[1 1 1] 양이 적은 경우
              (`/Game/CoreVR/Blueprints/Widget/UI_MenuInfo.LowLevel` _as_ui_menu_info)
              (`/Game/CoreVR/Blueprints/Widget/UI_MenuInfo.LowLevel` (`self.As UI Menu Info_0`))
              (`/Game/CoreVR/Blueprints/Widget/UI_MenuInfo.LowLevel` (`self.As UI Menu Info_1`))
              (`GameplayStatics.PlaySoundAtLocation` "/Game/CoreVR/Audio/Error_Cue.Error_Cue" (`self.K2_GetActorLocation`) (struct) 1.0 1.0 0.0 null null null null)
              (`KismetSystemLibrary.Delay` 0.5)
              (set `self.CallCooldown` false)))
          (elif (and (`|EnumEquality` (`self.Menu`) (`/Game/CoreVR/Blueprints/Tools_Liquid/BP_BaseCup.Now Type` _as_bp_test_cup)) (== (`/Game/CoreVR/Blueprints/Tools_Liquid/BP_BaseCup.Cream?` _as_bp_test_cup) (`self.Cream?`)) (== (`|EnumEquality` (`/Game/CoreVR/Blueprints/Tools_Liquid/BP_BaseCup.Temp` _as_bp_test_cup) "NewEnumerator14") (`self.Ice?`)))
            (goto _label)
            (else
              ;;[1 1 1] 일치하지 않는 경우
              (`/Game/CoreVR/Blueprints/Widget/UI_MenuInfo.Not Equal` _as_ui_menu_info :!label _label_2)
              (`/Game/CoreVR/Blueprints/Widget/UI_MenuInfo.Not Equal` (`self.As UI Menu Info_0`))
              (`/Game/CoreVR/Blueprints/Widget/UI_MenuInfo.Not Equal` (`self.As UI Menu Info_1`))
              (`GameplayStatics.PlaySoundAtLocation` "/Game/CoreVR/Audio/Error_Cue.Error_Cue" (`self.K2_GetActorLocation`) (struct) 1.0 1.0 0.0 null null null null)
              (`KismetSystemLibrary.Delay` 0.5)
              (set `self.CallCooldown` false)))))
      (:`else`
        (goto _label_2)))))

(fn `UserConstructionScript`)