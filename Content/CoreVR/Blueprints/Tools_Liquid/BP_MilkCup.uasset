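; BP_MilkCup is a VR milk cup that shows contextual prompts for milk steaming.
; Each tick, while held with Normal or Cold milk, it turns on the Steamer's attach-milk state, finding and caching BP_Steamer if needed.
; Releasing or emptying the cup clears that state and the press-button state.
; A camera-facing text label appears only when the held cup is empty.
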(event `self.ReceiveTick`
  (params (DeltaSeconds :type "Float (single-precision)"))
  (`parent.ReceiveTick` DeltaSeconds)
  (`|ExecutionSequence`
    (:`then_0`
      (if (`self.Grab?`)
        (if (> (`self.Now Amount`) 0.0)
          (`self.T_Milk` false)
          (switch `/Game/CoreVR/Blueprints/Tools_Liquid/E_Temp` (`self.Temp`)
            (:`NewEnumerator13`
              _)
            (:`NewEnumerator14`
              _))
          (bind _steamer (`self.Steamer`)
            (:`then`
              (`/Game/CoreVR/Blueprints/Tools_Maker/BP_Steamer.T_AttachMilk` _steamer true)
              (set `self.Show` true))
            (:`else`
              (bind _returnvalue (`GameplayStatics.GetActorOfClass` "/Game/CoreVR/Blueprints/Tools_Maker/BP_Steamer.BP_Steamer_C"))
              (bind _output_get (set `self.Steamer` _returnvalue))
              (`/Game/CoreVR/Blueprints/Tools_Maker/BP_Steamer.T_AttachMilk` _output_get true)
              (set `self.Show` true)))
          (else
            (`self.T_Milk` true)
            (if (`self.Show`) :!label _label
              (set `self.Show` false)
              (bind _steamer_2 (`self.Steamer`)
                (:`then`
                  (`/Game/CoreVR/Blueprints/Tools_Maker/BP_Steamer.T_AttachMilk` _steamer_2 false)
                  (`/Game/CoreVR/Blueprints/Tools_Maker/BP_Steamer.T_PressButton` _steamer_2 false))
                (:`else`
                  (bind _returnvalue_2 (`GameplayStatics.GetActorOfClass` "/Game/CoreVR/Blueprints/Tools_Maker/BP_Steamer.BP_Steamer_C"))
                  (bind _output_get_2 (set `self.Steamer` _returnvalue_2))
                  (`/Game/CoreVR/Blueprints/Tools_Maker/BP_Steamer.T_AttachMilk` _output_get_2 false)
                  (`/Game/CoreVR/Blueprints/Tools_Maker/BP_Steamer.T_PressButton` _output_get_2 false))))))
        (else
          (`self.T_Milk` false)
          (goto _label))))
    (:`then_1`
      (`SceneComponent.K2_SetWorldRotation` (`self.TextRender1`) (`KismetMathLibrary.FindLookAtRotation` (`SceneComponent.K2_GetComponentLocation` (`self.Cup`)) (`self.K2_GetActorLocation` (`PlayerController.PlayerCameraManager` (`GameplayStatics.GetPlayerController` 0)))) false false))))

(event `T_Milk`
  (params (bNewVisibility :type Boolean))
  (`SceneComponent.SetVisibility` (`self.TextRender1`) bNewVisibility false))

(fn `UserConstructionScript`
  (`parent.UserConstructionScript`))