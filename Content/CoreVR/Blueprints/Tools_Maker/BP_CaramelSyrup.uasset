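; BP_CaramelSyrup is a VR caramel syrup dispenser that gives a short, fixed dose of liquid to a cup.
; A hand-tagged component entering its Box triggers haptics, sound, button tint and particle flow, then starts a looping timer.
; Each tick line-traces from the Arrow and passes Liquid to any unfilled BP_BaseCup hit.
; After a few ticks the timer clears, resetting button and particles, and re-arming the trigger.
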(event `self.ReceiveBeginPlay`
  (bind _returnvalue (`PrimitiveComponent.CreateDynamicMaterialInstance` (`self.Cube1`) 0 "/Game/Asset/CustomMesh/Material/M_Button.M_Button" "None"))
  (set `self.MI_Button` _returnvalue))

(event `self.Box.OnComponentBeginOverlap`
  (params (OverlappedComponent :type "PrimitiveComponent Object Reference") (OtherActor :type "Actor Object Reference") (OtherComp :type "PrimitiveComponent Object Reference") (OtherBodyIndex :type Integer) (bFromSweep :type Boolean) (SweepResult :type "HitResult Structure (by ref)"))
  (bind _returnvalue (`GameplayStatics.GetPlayerController` 0))
  (if (`self.SetTimer`)
    _
    (elif (`ActorComponent.ComponentHasTag` OtherComp "Left")
      (`PlayerController.PlayHapticEffect` _returnvalue "/Game/CoreVR/Haptics/ButtonHapticEffect.ButtonHapticEffect" "Left" 0.5 false)
      (`MaterialInstanceDynamic.SetVectorParameterValue` (`self.MI_Button`) "Color" (struct :`R` 1.0 :`B` 0.045438 :`A` 1.0) :!label _label)
      (`self.FlowParticle?` true)
      (`GameplayStatics.PlaySoundAtLocation` "/Game/CoreVR/Audio/Syrup_Cue.Syrup_Cue" (`self.K2_GetActorLocation`) (struct) 1.0 1.0 0.0 null null null null)
      (set `self.NowFluid` 0)
      (bind _returnvalue_2 (`KismetSystemLibrary.K2_SetTimerDelegate` (delegate `Giving`) 0.1 true))
      (set `self.Timer` _returnvalue_2)
      (set `self.SetTimer` true)
      (elif (`ActorComponent.ComponentHasTag` OtherComp "Right")
        (`PlayerController.PlayHapticEffect` _returnvalue "/Game/CoreVR/Haptics/PistolFireHapticEffect.PistolFireHapticEffect" "Right" 0.5 false)
        (goto _label)))))

(event `Giving`
  (bind _returnvalue (`SceneComponent.K2_GetComponentLocation` (`self.Arrow`)))
  (bind _result (`/Engine/EditorBlueprintResources/StandardMacros.IncrementInt` (`self.NowFluid`))
    (:`  `
      (if (< _result 6)
        (bind (_outhit _returnvalue_2) (`KismetSystemLibrary.LineTraceSingleForObjects` _returnvalue (+ _returnvalue (* (`KismetMathLibrary.MakeRotator` 0.0 -90.0) 1000.0)) (`self.Object Types`)))
        (if _returnvalue_2
          (bind _asbp_base_cup (cast `/Game/CoreVR/Blueprints/Tools_Liquid/BP_BaseCup` (`.HitActor` (`GameplayStatics.BreakHitResult` _outhit)))
            (:`then`
              (`self.Give Fluid` _asbp_base_cup)
              (set `self.NowFlow?` true))
            (:`CastFailed`
              (set `self.NowFlow?` false)))
          (else
            (set `self.NowFlow?` false)))
        (else
          (`KismetSystemLibrary.K2_ClearAndInvalidateTimerHandle` (`self.Timer`))
          (set `self.SetTimer` false)
          (`MaterialInstanceDynamic.SetVectorParameterValue` (`self.MI_Button`) "Color" (struct :`R` 1.0 :`G` 1.0 :`B` 1.0 :`A` 1.0))
          (`self.FlowParticle?` false))))))

(event `FlowParticle?`
  (params (Condition :type Boolean))
  (bind _liquid1 (`self.Liquid1`))
  (if Condition
    (`FXSystemComponent.SetFloatParameter` _liquid1 "spawnrate" 20.0)
    (else
      (`FXSystemComponent.SetFloatParameter` _liquid1 "spawnrate" 0.0))))

(event `Give Fluid`
  (params (CupActor :type "/Game/CoreVR/Blueprints/Tools_Liquid/BP_BaseCup Object Reference"))
  ;[1 1 1] 현재 Liquid를 구성하고 있는 비율만큼 Liquid 제공
  (if (< (`/Game/CoreVR/Blueprints/Tools_Liquid/BP_BaseCup.Now Amount` CupActor) (`/Game/CoreVR/Blueprints/Tools_Liquid/BP_BaseCup.Max Amount` CupActor))
    (`/Game/CoreVR/Blueprints/Tools_Liquid/BP_BaseCup.Get Fluid` CupActor (`self.Liquid`))))

(fn `UserConstructionScript`)