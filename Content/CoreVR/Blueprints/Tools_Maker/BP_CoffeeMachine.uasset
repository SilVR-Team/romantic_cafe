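; VR coffee machine actor that takes a BP_Porta portafilter and dispenses liquid into cups.
; An overlapping portafilter snaps into its socket and updates prompt texts; a hand-tagged button touch starts brewing with haptics, sounds, indicator colors and flow particles.
; A fast looping timer line-traces for a BP_BaseCup, filling it with liquid chosen by portafilter state.
; After a fixed tick count, brewing stops and the portafilter state resets.
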(event `self.ReceiveBeginPlay`
  (bind _returnvalue (`PrimitiveComponent.CreateDynamicMaterialInstance` (`self.Cube1`) 0 "/Game/Asset/CustomMesh/Material/M_Button.M_Button" "None"))
  (set `self.MI_Button` _returnvalue)
  (bind _returnvalue_2 (`PrimitiveComponent.CreateDynamicMaterialInstance` (`self.Cylinder`) 0 "/Game/Asset/CustomMesh/Material/M_Button.M_Button" "None"))
  (set `self.MI_On` _returnvalue_2)
  (bind _returnvalue_3 (`PrimitiveComponent.CreateDynamicMaterialInstance` (`self.Cylinder1`) 0 "/Game/Asset/CustomMesh/Material/M_Button.M_Button" "None"))
  (set `self.MI_Off` _returnvalue_3)
  (`MaterialInstanceDynamic.SetVectorParameterValue` (`self.MI_Off`) "Color" (struct :`G` 1.0 :`A` 1.0))
  (`MaterialInstanceDynamic.SetVectorParameterValue` (`self.MI_On`) "Color" (struct :`A` 1.0))
  (`MaterialInstanceDynamic.SetVectorParameterValue` (`self.MI_Button`) "Color" (struct :`R` 1.0 :`A` 1.0)))

(event `self.Sphere.OnComponentBeginOverlap`
  (params (OverlappedComponent :type "PrimitiveComponent Object Reference") (OtherActor :type "Actor Object Reference") (OtherComp :type "PrimitiveComponent Object Reference") (OtherBodyIndex :type Integer) (bFromSweep :type Boolean) (SweepResult :type "HitResult Structure (by ref)"))
  (bind _asbp_porta (cast `/Game/CoreVR/Blueprints/Tools_Maker/BP_Porta` OtherActor))
  (bind _output_get (set `self.As BP Porta` _asbp_porta))
  (`self.K2_AttachToComponent` _output_get (`self.Socket_Porta`) "None" "SnapToTarget" "SnapToTarget" "SnapToTarget" true)
  (set `/Game/CoreVR/Blueprints/Tools_Maker/BP_Porta.Attached?` true _output_get)
  (`PlayerController.PlayHapticEffect` (`GameplayStatics.GetPlayerController` 0) "/Game/CoreVR/Haptics/AttachHapticEffect.AttachHapticEffect" (`/Game/CoreVR/Blueprints/Component/BP_GrabComponent.GetHeldByHand` (`/Game/CoreVR/Blueprints/Tools_Maker/BP_Porta.GrabComponent` _output_get)) 0.5 false)
  (`GameplayStatics.PlaySoundAtLocation` "/Game/CoreVR/Audio/chulkuck_Cue.chulkuck_Cue" (`self.K2_GetActorLocation`) (struct) 1.0 1.0 0.0 null null null null)
  (`self.T_PressButton` true)
  (`self.T_Attach_Filter` false))

(event `self.Sphere.OnComponentEndOverlap`
  (params (OverlappedComponent :type "PrimitiveComponent Object Reference") (OtherActor :type "Actor Object Reference") (OtherComp :type "PrimitiveComponent Object Reference") (OtherBodyIndex :type Integer))
  (if (== OtherActor (`self.As BP Porta`))
    (set `/Game/CoreVR/Blueprints/Tools_Maker/BP_Porta.Attached?` false (`self.As BP Porta`))
    (set `self.As BP Porta` null)
    (`self.T_PressButton` false)))

(event `self.Box.OnComponentBeginOverlap`
  (params (OverlappedComponent :type "PrimitiveComponent Object Reference") (OtherActor :type "Actor Object Reference") (OtherComp :type "PrimitiveComponent Object Reference") (OtherBodyIndex :type Integer) (bFromSweep :type Boolean) (SweepResult :type "HitResult Structure (by ref)"))
  (bind _returnvalue (`GameplayStatics.GetPlayerController` 0))
  (if (`self.SetTimer`)
    _
    (elif (`ActorComponent.ComponentHasTag` OtherComp "Left")
      (`PlayerController.PlayHapticEffect` _returnvalue "/Game/CoreVR/Haptics/ButtonHapticEffect.ButtonHapticEffect" "Left" 0.5 false)
      (`MaterialInstanceDynamic.SetVectorParameterValue` (`self.MI_Button`) "Color" (struct :`R` 1.0 :`G` 1.0 :`B` 1.0 :`A` 1.0) :!label _label)
      (`KismetSystemLibrary.Delay` 0.5)
      (`GameplayStatics.PlaySoundAtLocation` "/Game/CoreVR/Audio/CoffeeMachine_ON_Cue.CoffeeMachine_ON_Cue" (`self.K2_GetActorLocation`) (struct) 1.0 1.0 0.0 null null null null)
      (`MaterialInstanceDynamic.SetVectorParameterValue` (`self.MI_Button`) "Color" (struct :`R` 1.0 :`A` 1.0))
      (`MaterialInstanceDynamic.SetVectorParameterValue` (`self.MI_On`) "Color" (struct :`R` 1.0 :`A` 1.0))
      (`MaterialInstanceDynamic.SetVectorParameterValue` (`self.MI_Off`) "Color" (struct :`A` 1.0))
      (`GameplayStatics.PlaySoundAtLocation` "/Game/CoreVR/Audio/CoffeeMachine_Cue.CoffeeMachine_Cue" (`self.K2_GetActorLocation`) (struct) 1.0 1.0 0.0 null null null null)
      (set `self.NowFluid` 0)
      (bind _returnvalue_2 (`KismetSystemLibrary.K2_SetTimerDelegate` (delegate `Giving`) 0.005 true))
      (set `self.Timer` _returnvalue_2)
      (set `self.SetTimer` true)
      (`self.FlowParticle?` true)
      (bind _as_bp_porta (`self.As BP Porta`)
        (:`then`
          (`/Game/CoreVR/Blueprints/Tools_Maker/BP_Porta.Using` _as_bp_porta true)
          (`self.T_PressButton` false))
        (:`else`))
      (elif (`ActorComponent.ComponentHasTag` OtherComp "Right")
        (`PlayerController.PlayHapticEffect` _returnvalue "/Game/CoreVR/Haptics/PistolFireHapticEffect.PistolFireHapticEffect" "Right" 0.5 false)
        (goto _label)))))

(event `Giving`
  (bind _as_bp_porta (`self.As BP Porta`))
  (bind _returnvalue (`SceneComponent.K2_GetComponentLocation` (`self.Arrow`)))
  (bind _result (`/Engine/EditorBlueprintResources/StandardMacros.IncrementInt` (`self.NowFluid`))
    (:`  `
      (if (< _result 4002)
        (bind (_outhit _returnvalue_2) (`KismetSystemLibrary.LineTraceSingleForObjects` _returnvalue (+ _returnvalue (* (`KismetMathLibrary.MakeRotator` 0.0 -90.0) 1000.0)) (`self.Object Types`)))
        (if _returnvalue_2
          (bind _asbp_base_cup (cast `/Game/CoreVR/Blueprints/Tools_Liquid/BP_BaseCup` (`.HitActor` (`GameplayStatics.BreakHitResult` _outhit)))
            (:`then`
              (`self.Give Fluid` _asbp_base_cup)
              (set `self.NowFlow?` true)
              (`/Game/CoreVR/Blueprints/Tools_Liquid/BP_BaseCup.Get Cream` _asbp_base_cup false))
            (:`CastFailed`
              (set `self.NowFlow?` false)))
          (else
            (set `self.NowFlow?` false)))
        (else
          (`KismetSystemLibrary.K2_ClearAndInvalidateTimerHandle` (`self.Timer`))
          (set `self.SetTimer` false)
          (`MaterialInstanceDynamic.SetVectorParameterValue` (`self.MI_Off`) "Color" (struct :`G` 1.0 :`A` 1.0))
          (`MaterialInstanceDynamic.SetVectorParameterValue` (`self.MI_On`) "Color" (struct :`A` 1.0))
          (`self.FlowParticle?` false)
          (`self.As BP Porta`
            (:`then`
              (`/Game/CoreVR/Blueprints/Tools_Maker/BP_Porta.Set State` _as_bp_porta "NewEnumerator0")
              (`/Game/CoreVR/Blueprints/Tools_Maker/BP_Porta.Using` _as_bp_porta false))
            (:`else`
              _))
          (`KismetSystemLibrary.Delay` 0.5)
          (`GameplayStatics.PlaySoundAtLocation` "/Game/CoreVR/Audio/CoffeeMachine_OFF_Cue.CoffeeMachine_OFF_Cue" (`self.K2_GetActorLocation`) (struct) 1.0 1.0 0.0 null null null null))))))

(event `T_Attach_Filter`
  (params (bNewVisibility :type Boolean))
  (`SceneComponent.SetVisibility` (`self.TextRender1`) bNewVisibility false))

(event `T_PressButton`
  (params (bNewVisibility :type Boolean))
  (`SceneComponent.SetVisibility` (`self.TextRender2`) bNewVisibility false))

(event `Give Fluid`
  (params (CupActor :type "/Game/CoreVR/Blueprints/Tools_Liquid/BP_BaseCup Object Reference"))
  ;[1 1 1] 현재 Liquid를 구성하고 있는 비율만큼 Liquid 제공
  (if (< (`/Game/CoreVR/Blueprints/Tools_Liquid/BP_BaseCup.Now Amount` CupActor) (`/Game/CoreVR/Blueprints/Tools_Liquid/BP_BaseCup.Max Amount` CupActor))
    (bind _as_bp_porta (`self.As BP Porta`)
      (:`then`
        (bind _state (`/Game/CoreVR/Blueprints/Tools_Maker/BP_Porta.State` _as_bp_porta))
        (if (`|EnumEquality` _state "NewEnumerator2")
          (`/Game/CoreVR/Blueprints/Tools_Liquid/BP_BaseCup.Get Fluid` CupActor (`self.Liquid`))
          (elif (`|EnumEquality` _state "NewEnumerator1")
            (`/Game/CoreVR/Blueprints/Tools_Liquid/BP_BaseCup.Get Fluid` CupActor (`self.Liquid_1`))
            (else
              (`/Game/CoreVR/Blueprints/Tools_Liquid/BP_BaseCup.Get Fluid` CupActor (`self.Liquid_2`) :!label _label_2)))))
      (:`else`
        (goto _label_2)))))

(event `FlowParticle?`
  (params (Condition :type Boolean))
  (bind _liquid1 (`self.Liquid1`))
  (if Condition
    (`FXSystemComponent.SetFloatParameter` _liquid1 "spawnrate" 30.0)
    (`FXSystemComponent.SetFloatParameter` (`self.Liquid2`) "spawnrate" 30.0)
    (else
      (`FXSystemComponent.SetFloatParameter` _liquid1 "spawnrate" 0.0)
      (`FXSystemComponent.SetFloatParameter` (`self.Liquid2`) "spawnrate" 0.0))))

(fn `UserConstructionScript`)