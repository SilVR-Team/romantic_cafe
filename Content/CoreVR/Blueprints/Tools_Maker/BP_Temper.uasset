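; BP_Temper is a grabbable VR temper tool with a text prompt that turns toward the player camera every tick.
; T_TakeTemper shows or hides the prompt; grabbing hides it and, if it was visible, calls TTemping(true) on BP_TempingMat.
; Dropping restores the saved visibility and calls TTemping(false).
; Overlapping a BP_ResetArea briefly disables physics to return the mesh to its BeginPlay transform.
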(event `self.ReceiveBeginPlay`
  (set `self.Origin` (`SceneComponent.K2_GetComponentToWorld` (`self.StaticMesh`))))

(event `self.StaticMesh.OnComponentBeginOverlap`
  (params (OverlappedComponent :type "PrimitiveComponent Object Reference") (OtherActor :type "Actor Object Reference") (OtherComp :type "PrimitiveComponent Object Reference") (OtherBodyIndex :type Integer) (bFromSweep :type Boolean) (SweepResult :type "HitResult Structure (by ref)"))
  (bind _staticmesh (`self.StaticMesh`))
  (bind (_origin_location _origin_rotation _origin_scale) (`KismetMathLibrary.BreakTransform` (`self.Origin`)))
  (cast `/Game/CoreVR/Blueprints/Tools_Game/BP_ResetArea` OtherActor)
  (`PrimitiveComponent.SetSimulatePhysics` _staticmesh false)
  (`SceneComponent.K2_SetWorldTransform` (`self.StaticMesh`) (`KismetMathLibrary.MakeTransform` _origin_location _origin_rotation _origin_scale) false false)
  (`PrimitiveComponent.SetSimulatePhysics` _staticmesh true))

(event `self.ReceiveTick`
  (params (DeltaSeconds :type "Float (single-precision)"))
  (`SceneComponent.K2_SetWorldRotation` (`self.TextRender1`) (`KismetMathLibrary.FindLookAtRotation` (`SceneComponent.K2_GetComponentLocation` (`self.StaticMesh`)) (`self.K2_GetActorLocation` (`PlayerController.PlayerCameraManager` (`GameplayStatics.GetPlayerController` 0)))) false false))

(event `T_TakeTemper`
  (params (bNewVisibility :type Boolean))
  (`SceneComponent.SetVisibility` (`self.TextRender1`) bNewVisibility false)
  (set `self.RecentVisible` bNewVisibility))

(event `self.GrabComponent.OnGrabbed`
  (bind _bvisible (`SceneComponent.bVisible` (`self.TextRender1`)))
  (set `self.RecentVisible` _bvisible)
  (if _bvisible
    (`SceneComponent.SetVisibility` (`self.TextRender1`) false false)
    (bind _returnvalue (`GameplayStatics.GetActorOfClass` "/Game/CoreVR/Blueprints/Tools_Maker/BP_TempingMat.BP_TempingMat_C"))
    (`/Game/CoreVR/Blueprints/Tools_Maker/BP_TempingMat.T_Temping` _returnvalue true)))

(event `self.GrabComponent.OnDropped`
  (if (`self.RecentVisible`)
    (`SceneComponent.SetVisibility` (`self.TextRender1`) true false)
    (bind _returnvalue (`GameplayStatics.GetActorOfClass` "/Game/CoreVR/Blueprints/Tools_Maker/BP_TempingMat.BP_TempingMat_C"))
    (`/Game/CoreVR/Blueprints/Tools_Maker/BP_TempingMat.T_Temping` _returnvalue false)
    (else
      (`SceneComponent.SetVisibility` (`self.TextRender1`) false false)
      (bind _returnvalue_2 (`GameplayStatics.GetActorOfClass` "/Game/CoreVR/Blueprints/Tools_Maker/BP_TempingMat.BP_TempingMat_C"))
      (`/Game/CoreVR/Blueprints/Tools_Maker/BP_TempingMat.T_Temping` _returnvalue_2 false))))

(fn `UserConstructionScript`)