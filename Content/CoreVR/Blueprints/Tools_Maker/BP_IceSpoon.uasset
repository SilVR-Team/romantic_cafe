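; VR ice scoop tool that carries ice and tips it into cups.
; Getice shows the ice mesh; while loaded, Tick checks the scoop's tilt and line-traces down from FlowStartPoint for a BP_BaseCup.
; Cups that accept ice receive it and sinks discard it, emptying the scoop with a sound; other restricted cups leave it full.
; Overlapping a BP_ResetArea returns the physics body to its BeginPlay transform.
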(event `self.ReceiveBeginPlay`
  ;[1 1 1] 테스트용 변수 설정
  (set `self.Origin` (`SceneComponent.K2_GetComponentToWorld` (`self.Cube`))))

(event `self.ReceiveTick`
  (params (DeltaSeconds :type "Float (single-precision)"))
  (bind (_returnvalue_roll _returnvalue_pitch) (`KismetMathLibrary.BreakRotator` (`SceneComponent.K2_GetComponentRotation` (`self.Cube`))))
  (bind _returnvalue (`SceneComponent.K2_GetComponentLocation` (`self.FlowStartPoint`)))
  ;[1 1 1] 기울기 & 컵 인식
  (if (and (`self.Ice?`) (or (>= (`KismetMathLibrary.Abs` _returnvalue_roll) 90.0) (<= _returnvalue_pitch -10.0)))
    (bind (_outhit _returnvalue_2) (`KismetSystemLibrary.LineTraceSingleForObjects` _returnvalue (+ _returnvalue (* (`KismetMathLibrary.MakeRotator` 0.0 -90.0) 1000.0)) (`self.Object Types`)))
    (if _returnvalue_2
      (bind _asbp_base_cup (cast `/Game/CoreVR/Blueprints/Tools_Liquid/BP_BaseCup` (`.HitActor` (`GameplayStatics.BreakHitResult` _outhit))))
      (if (or (`/Game/CoreVR/Blueprints/Tools_Liquid/BP_BaseCup.UseOnly` _asbp_base_cup) (`/Game/CoreVR/Blueprints/Tools_Liquid/BP_BaseCup.MilkOnly` _asbp_base_cup) (`/Game/CoreVR/Blueprints/Tools_Liquid/BP_BaseCup.NoIce` _asbp_base_cup))
        (if (`/Game/CoreVR/Blueprints/Tools_Liquid/BP_BaseCup.Sink` _asbp_base_cup)
          (set `self.Ice?` false :!label _label)
          (`SceneComponent.SetVisibility` (`self.Cube1`) false false)
          (`GameplayStatics.PlaySoundAtLocation` "/Game/CoreVR/Audio/Ice_In_Cue.Ice_In_Cue" (`self.K2_GetActorLocation`) (struct) 1.0 1.0 0.0 null null null null))
        (else
          (`/Game/CoreVR/Blueprints/Tools_Liquid/BP_BaseCup.Get Ice` _asbp_base_cup)
          (goto _label))))))

(event `Get ice`
  (set `self.Ice?` true)
  (`SceneComponent.SetVisibility` (`self.Cube1`) true false)
  (`GameplayStatics.PlaySoundAtLocation` "/Game/CoreVR/Audio/GetIce_Cue.GetIce_Cue" (`self.K2_GetActorLocation`) (struct) 1.0 1.0 0.0 null null null null))

(event `self.Cube.OnComponentBeginOverlap`
  (params (OverlappedComponent :type "PrimitiveComponent Object Reference") (OtherActor :type "Actor Object Reference") (OtherComp :type "PrimitiveComponent Object Reference") (OtherBodyIndex :type Integer) (bFromSweep :type Boolean) (SweepResult :type "HitResult Structure (by ref)"))
  (bind (_origin_location _origin_rotation _origin_scale) (`KismetMathLibrary.BreakTransform` (`self.Origin`)))
  (bind _cube (`self.Cube`))
  (cast `/Game/CoreVR/Blueprints/Tools_Game/BP_ResetArea` OtherActor)
  (`PrimitiveComponent.SetSimulatePhysics` _cube false)
  (`SceneComponent.K2_SetWorldTransform` _cube (`KismetMathLibrary.MakeTransform` _origin_location _origin_rotation _origin_scale) false false)
  (`PrimitiveComponent.SetSimulatePhysics` (`self.Cube`) true))

(fn `UserConstructionScript`)