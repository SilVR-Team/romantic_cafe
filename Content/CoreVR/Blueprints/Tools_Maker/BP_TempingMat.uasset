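; VR tamping mat that takes a portafilter (BP_Porta) and tamps it with a BP_Temper tool, apparently for coffee making.
; A sphere overlap snaps the portafilter to a socket, then tool contact switches it from UnTempered to Tempered with sound and haptics.
; Three text renders act as step prompts, coordinated with the tamper's own prompt via GetActorOfClass.
; Ending the portafilter's overlap clears the reference and hides the take prompts.
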(event `self.Sphere.OnComponentBeginOverlap`
  (params (OverlappedComponent :type "PrimitiveComponent Object Reference") (OtherActor :type "Actor Object Reference") (OtherComp :type "PrimitiveComponent Object Reference") (OtherBodyIndex :type Integer) (bFromSweep :type Boolean) (SweepResult :type "HitResult Structure (by ref)"))
  (bind _as_bp_porta (`self.As BP Porta`))
  (bind _asbp_porta (cast `/Game/CoreVR/Blueprints/Tools_Maker/BP_Porta` OtherActor)
    (:`then`
      (bind _output_get (set `self.As BP Porta` _asbp_porta))
      (`self.K2_AttachToComponent` _output_get (`self.Socket_Porta`) "None" "SnapToTarget" "SnapToTarget" "SnapToTarget" true)
      (set `/Game/CoreVR/Blueprints/Tools_Maker/BP_Porta.Attached?` true _output_get)
      (`PlayerController.PlayHapticEffect` (`GameplayStatics.GetPlayerController` 0) "/Game/CoreVR/Haptics/AttachHapticEffect.AttachHapticEffect" (`/Game/CoreVR/Blueprints/Component/BP_GrabComponent.GetHeldByHand` (`/Game/CoreVR/Blueprints/Tools_Maker/BP_Porta.GrabComponent` _output_get)) 0.5 false)
      (`self.T_Attach_Filter` false)
      (switch `/Game/CoreVR/Blueprints/Tools_Maker/E_Porta` (`/Game/CoreVR/Blueprints/Tools_Maker/BP_Porta.State` (`self.As BP Porta`))
        (:`NewEnumerator1`
          (bind _returnvalue (`GameplayStatics.GetActorOfClass` "/Game/CoreVR/Blueprints/Tools_Maker/BP_Temper.BP_Temper_C"))
          (`/Game/CoreVR/Blueprints/Tools_Maker/BP_Temper.T_TakeTemper` _returnvalue true))
        (:`NewEnumerator2`
          (`self.T_Take` true))))
    (:`CastFailed`
      (cast `/Game/CoreVR/Blueprints/Tools_Maker/BP_Temper` OtherActor)
      (`/Engine/EditorBlueprintResources/StandardMacros.IsValid` _as_bp_porta
        (:`Is Valid`
          (if (`|EnumEquality` (`/Game/CoreVR/Blueprints/Tools_Maker/BP_Porta.State` _as_bp_porta) "NewEnumerator1")
            (`/Game/CoreVR/Blueprints/Tools_Maker/BP_Porta.Set State` _as_bp_porta "NewEnumerator2")
            (`PlayerController.PlayHapticEffect` (`GameplayStatics.GetPlayerController` 0) "/Game/CoreVR/Haptics/AttachHapticEffect.AttachHapticEffect" (`/Game/CoreVR/Blueprints/Component/BP_GrabComponent.GetHeldByHand` (`/Game/CoreVR/Blueprints/Tools_Maker/BP_Porta.GrabComponent` _as_bp_porta)) 0.5 false)
            (`GameplayStatics.PlaySoundAtLocation` "/Game/CoreVR/Audio/Temp.Temp" (`self.K2_GetActorLocation`) (struct) 1.0 1.0 0.0 null null null null)
            (`self.T_Take` true)
            (bind _returnvalue_2 (`GameplayStatics.GetActorOfClass` "/Game/CoreVR/Blueprints/Tools_Maker/BP_Temper.BP_Temper_C"))
            (`/Game/CoreVR/Blueprints/Tools_Maker/BP_Temper.T_TakeTemper` _returnvalue_2 false)
            (`self.T_Temping` false)))))))

(event `self.Sphere.OnComponentEndOverlap`
  (params (OverlappedComponent :type "PrimitiveComponent Object Reference") (OtherActor :type "Actor Object Reference") (OtherComp :type "PrimitiveComponent Object Reference") (OtherBodyIndex :type Integer))
  (if (== OtherActor (`self.As BP Porta`))
    (set `/Game/CoreVR/Blueprints/Tools_Maker/BP_Porta.Attached?` false (`self.As BP Porta`))
    (set `self.As BP Porta` null)
    (bind _returnvalue (`GameplayStatics.GetActorOfClass` "/Game/CoreVR/Blueprints/Tools_Maker/BP_Temper.BP_Temper_C"))
    (`/Game/CoreVR/Blueprints/Tools_Maker/BP_Temper.T_TakeTemper` _returnvalue false)
    (`self.T_Take` false)))

(event `T_Attach_Filter`
  (params (bNewVisibility :type Boolean))
  (`SceneComponent.SetVisibility` (`self.TextRender1`) bNewVisibility false))

(event `T_Temping`
  (params (bNewVisibility :type Boolean))
  (if bNewVisibility
    (switch `/Game/CoreVR/Blueprints/Tools_Maker/E_Porta` (`/Game/CoreVR/Blueprints/Tools_Maker/BP_Porta.State` (`self.As BP Porta`))
      (:`NewEnumerator1`
        (`SceneComponent.SetVisibility` (`self.TextRender2`) true false)))
    (else
      (`SceneComponent.SetVisibility` (`self.TextRender2`) bNewVisibility false))))

(event `T_Take`
  (params (bNewVisibility :type Boolean))
  (`SceneComponent.SetVisibility` (`self.TextRender3`) bNewVisibility false))

(fn `UserConstructionScript`)