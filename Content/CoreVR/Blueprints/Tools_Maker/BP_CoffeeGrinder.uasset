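; VR coffee grinder station that docks a BP_Porta portafilter and grinds into it at a button press.
; A sphere overlap snaps the porta to a socket with haptics and sound, then shows a press or detach prompt based on its state.
; A tagged hand touching the button box changes the button color and, with a porta docked, plays grinding for a fixed delay, sets it UnTempered and prompts detaching.
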(event `self.ReceiveBeginPlay`
  (bind _returnvalue (`PrimitiveComponent.CreateDynamicMaterialInstance` (`self.Cube1`) 0 "/Game/Asset/CustomMesh/Material/M_Button.M_Button" "None"))
  (set `self.MI_Button` _returnvalue)
  (`MaterialInstanceDynamic.SetVectorParameterValue` (`self.MI_Button`) "Color" (struct :`R` 1.0 :`A` 1.0)))

(event `self.Sphere.OnComponentBeginOverlap`
  (params (OverlappedComponent :type "PrimitiveComponent Object Reference") (OtherActor :type "Actor Object Reference") (OtherComp :type "PrimitiveComponent Object Reference") (OtherBodyIndex :type Integer) (bFromSweep :type Boolean) (SweepResult :type "HitResult Structure (by ref)"))
  (bind _asbp_porta (cast `/Game/CoreVR/Blueprints/Tools_Maker/BP_Porta` OtherActor))
  (bind _output_get (set `self.As BP Porta` _asbp_porta))
  (`self.K2_AttachToComponent` _output_get (`self.Socket_Porta`) "None" "SnapToTarget" "SnapToTarget" "SnapToTarget" true)
  (set `/Game/CoreVR/Blueprints/Tools_Maker/BP_Porta.Attached?` true _output_get)
  (`PlayerController.PlayHapticEffect` (`GameplayStatics.GetPlayerController` 0) "/Game/CoreVR/Haptics/AttachHapticEffect.AttachHapticEffect" (`/Game/CoreVR/Blueprints/Component/BP_GrabComponent.GetHeldByHand` (`/Game/CoreVR/Blueprints/Tools_Maker/BP_Porta.GrabComponent` _output_get)) 0.5 false)
  (`GameplayStatics.PlaySoundAtLocation` "/Game/CoreVR/Audio/chulkuck_Cue.chulkuck_Cue" (`self.K2_GetActorLocation`) (struct) 1.0 1.0 0.0 null null null null)
  (`self.T_Attach_Filter` false)
  (switch `/Game/CoreVR/Blueprints/Tools_Maker/E_Porta` (`/Game/CoreVR/Blueprints/Tools_Maker/BP_Porta.State` (`self.As BP Porta`))
    (:`NewEnumerator0`
      (`self.T_PressButton` true))
    (:`NewEnumerator1`
      (`self.T_Detach_Filter` true :!label _label))
    (:`NewEnumerator2`
      (goto _label))))

(event `self.Sphere.OnComponentEndOverlap`
  (params (OverlappedComponent :type "PrimitiveComponent Object Reference") (OtherActor :type "Actor Object Reference") (OtherComp :type "PrimitiveComponent Object Reference") (OtherBodyIndex :type Integer))
  (if (== OtherActor (`self.As BP Porta`))
    (set `/Game/CoreVR/Blueprints/Tools_Maker/BP_Porta.Attached?` false (`self.As BP Porta`))
    (set `self.As BP Porta` null)
    (`self.T_PressButton` false)
    (`self.T_Detach_Filter` false)))

(event `self.Box.OnComponentBeginOverlap`
  (params (OverlappedComponent :type "PrimitiveComponent Object Reference") (OtherActor :type "Actor Object Reference") (OtherComp :type "PrimitiveComponent Object Reference") (OtherBodyIndex :type Integer) (bFromSweep :type Boolean) (SweepResult :type "HitResult Structure (by ref)"))
  (bind _returnvalue (`GameplayStatics.GetPlayerController` 0))
  (bind _as_bp_porta (`self.As BP Porta`))
  (if (`self.On?`)
    (set `self.On?` false)
    (if (`ActorComponent.ComponentHasTag` OtherComp "Left")
      (`PlayerController.PlayHapticEffect` _returnvalue "/Game/CoreVR/Haptics/ButtonHapticEffect.ButtonHapticEffect" "Left" 0.5 false)
      (`MaterialInstanceDynamic.SetVectorParameterValue` (`self.MI_Button`) "Color" (struct :`R` 1.0 :`G` 1.0 :`B` 1.0 :`A` 1.0) :!label _label_2)
      (bind _as_bp_porta_2 (`self.As BP Porta`)
        (:`then`
          (`/Game/CoreVR/Blueprints/Tools_Maker/BP_Porta.Using` _as_bp_porta_2 true)
          (`GameplayStatics.PlaySoundAtLocation` "/Game/CoreVR/Audio/Grinder_Cue.Grinder_Cue" (`self.K2_GetActorLocation`) (struct) 1.0 1.0 0.0 null null null null)
          (`self.T_PressButton` false)
          (`KismetSystemLibrary.Delay` 3.0))
        (:`else`
          _))
      (set `self.On?` true)
      (`MaterialInstanceDynamic.SetVectorParameterValue` (`self.MI_Button`) "Color" (struct :`R` 1.0 :`A` 1.0))
      (`/Engine/EditorBlueprintResources/StandardMacros.IsValid` _as_bp_porta
        (:`Is Valid`
          (`/Game/CoreVR/Blueprints/Tools_Maker/BP_Porta.Set State` _as_bp_porta "NewEnumerator1")
          (bind _as_bp_porta_3 (`self.As BP Porta`)
            (:`then`
              (`/Game/CoreVR/Blueprints/Tools_Maker/BP_Porta.Using` _as_bp_porta_3 false)
              (`self.T_Detach_Filter` true))
            (:`else`))))
      (elif (`ActorComponent.ComponentHasTag` OtherComp "Right")
        (`PlayerController.PlayHapticEffect` _returnvalue "/Game/CoreVR/Haptics/PistolFireHapticEffect.PistolFireHapticEffect" "Right" 0.5 false)
        (goto _label_2)
        (else
          (set `self.On?` true))))))

(event `T_Attach_Filter`
  (params (bNewVisibility :type Boolean))
  (`SceneComponent.SetVisibility` (`self.TextRender1`) bNewVisibility false))

(event `T_PressButton`
  (params (bNewVisibility :type Boolean))
  (`SceneComponent.SetVisibility` (`self.TextRender2`) bNewVisibility false))

(event `T_Detach_Filter`
  (params (bNewVisibility :type Boolean))
  (`SceneComponent.SetVisibility` (`self.TextRender3`) bNewVisibility false))

(fn `UserConstructionScript`)