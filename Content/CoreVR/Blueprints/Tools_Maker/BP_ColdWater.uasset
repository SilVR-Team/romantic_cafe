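; Cold water dispenser for VR drink making, toggled by touching its button with a tagged left or right hand.
; A press plays haptics, sound and Niagara-style flow particles, stopping on another press or after 12 seconds, with a short debounce between presses.
; While on, a looping timer line-traces from the arrow and feeds Liquid to any BP_BaseCup hit that is below its maximum amount.
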(event `self.ReceiveBeginPlay`
  (bind _returnvalue (`PrimitiveComponent.CreateDynamicMaterialInstance` (`self.Cube1`) 0 "/Game/Asset/CustomMesh/Material/M_Button.M_Button" "None"))
  (bind _output_get (set `self.MI_Button` _returnvalue))
  (`MaterialInstanceDynamic.SetVectorParameterValue` _output_get "Color" (struct :`B` 1.0 :`A` 1.0)))

(event `self.Box.OnComponentBeginOverlap`
  (params (OverlappedComponent :type "PrimitiveComponent Object Reference") (OtherActor :type "Actor Object Reference") (OtherComp :type "PrimitiveComponent Object Reference") (OtherBodyIndex :type Integer) (bFromSweep :type Boolean) (SweepResult :type "HitResult Structure (by ref)"))
  (bind _returnvalue (`GameplayStatics.GetPlayerController` 0))
  (if (`self.Switch`)
    (set `self.Switch` false)
    (`|ExecutionSequence`
      (:`then_0`
        (if (`ActorComponent.ComponentHasTag` OtherComp "Left")
          (`PlayerController.PlayHapticEffect` _returnvalue "/Game/CoreVR/Haptics/ButtonHapticEffect.ButtonHapticEffect" "Left" 0.5 false)
          (`MaterialInstanceDynamic.SetVectorParameterValue` (`self.MI_Button`) "Color" (struct :`R` 1.0 :`G` 1.0 :`B` 1.0 :`A` 1.0) :!label _label)
          (if (not (`self.ON?`))
            (bind _returnvalue_2 (`GameplayStatics.SpawnSoundAttached` "/Game/CoreVR/Audio/Water_Cue.Water_Cue" (`self.Cube`) "None" (0.0 0.0 0.0) (struct) "KeepRelativeOffset" false 1.0 1.0 0.0 null null))
            (bind _output_get (set `self.Sound` _returnvalue_2))
            (`AudioComponent.FadeIn` _output_get 0.5 1.0 0.0 "Linear")
            (set `self.ON?` true)
            (`GameplayStatics.PlaySoundAtLocation` "/Game/CoreVR/Audio/Water_ON_Cue.Water_ON_Cue" (`self.K2_GetActorLocation`) (struct) 1.0 1.0 0.0 null null null null)
            (bind _returnvalue_3 (`KismetSystemLibrary.K2_SetTimerDelegate` (delegate `Giving`) 0.1 true))
            (set `self.Timer` _returnvalue_3)
            (`self.FlowParticle?` true)
            (`KismetSystemLibrary.RetriggerableDelay` 12.0))
          (`KismetSystemLibrary.K2_ClearAndInvalidateTimerHandle` (`self.Timer`))
          (if (`self.ON?`)
            (`MaterialInstanceDynamic.SetVectorParameterValue` (`self.MI_Button`) "Color" (struct :`B` 1.0 :`A` 1.0))
            (set `self.ON?` false)
            (`self.FlowParticle?` false)
            (`GameplayStatics.PlaySoundAtLocation` "/Game/CoreVR/Audio/Water_OFF_Cue.Water_OFF_Cue" (`self.K2_GetActorLocation`) (struct) 1.0 1.0 0.0 null null null null)
            (bind _sound (`self.Sound`)
              (:`then`
                (`AudioComponent.FadeOut` _sound 0.1 0.0 "Linear"))
              (:`else`)))
          (elif (`ActorComponent.ComponentHasTag` OtherComp "Right")
            (`PlayerController.PlayHapticEffect` _returnvalue "/Game/CoreVR/Haptics/PistolFireHapticEffect.PistolFireHapticEffect" "Right" 0.5 false)
            (goto _label))))
      (:`then_1`
        (`KismetSystemLibrary.Delay` 0.5)
        (set `self.Switch` true)))))

(event `Giving`
  (bind _returnvalue (`SceneComponent.K2_GetComponentLocation` (`self.Arrow`)))
  (bind (_outhit _returnvalue_2) (`KismetSystemLibrary.LineTraceSingleForObjects` _returnvalue (+ _returnvalue (* (`KismetMathLibrary.MakeRotator` 0.0 -90.0) 1000.0)) (`self.Object Types`)))
  (if _returnvalue_2
    (bind _asbp_base_cup (cast `/Game/CoreVR/Blueprints/Tools_Liquid/BP_BaseCup` (`.HitActor` (`GameplayStatics.BreakHitResult` _outhit)))
      (:`then`
        (`self.Give Fluid` _asbp_base_cup)
        (set `self.NowFlow?` true)
        (`/Game/CoreVR/Blueprints/Tools_Liquid/BP_BaseCup.Get Cream` _asbp_base_cup false))
      (:`CastFailed`
        (set `self.NowFlow?` false)))
    (else
      (set `self.NowFlow?` false))))

(event `Give Fluid`
  (params (CupActor :type "/Game/CoreVR/Blueprints/Tools_Liquid/BP_BaseCup Object Reference"))
  ;[1 1 1] 현재 Liquid를 구성하고 있는 비율만큼 Liquid 제공
  (if (< (`/Game/CoreVR/Blueprints/Tools_Liquid/BP_BaseCup.Now Amount` CupActor) (`/Game/CoreVR/Blueprints/Tools_Liquid/BP_BaseCup.Max Amount` CupActor))
    (`/Game/CoreVR/Blueprints/Tools_Liquid/BP_BaseCup.Get Fluid` CupActor (`self.Liquid`))))

(event `FlowParticle?`
  (params (Condition :type Boolean))
  (bind _liquid1 (`self.Liquid1`))
  (if Condition
    (`FXSystemComponent.SetFloatParameter` _liquid1 "spawnrate" 200.0)
    (else
      (`FXSystemComponent.SetFloatParameter` _liquid1 "spawnrate" 0.0))))

(fn `UserConstructionScript`)