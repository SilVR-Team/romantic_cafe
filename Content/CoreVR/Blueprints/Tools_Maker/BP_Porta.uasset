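; BP_Porta is a grabbable VR coffee portafilter with Clear, Un Tempered and Tempered states, shown by toggling the tamped-coffee visuals.
; On grab, its state picks whether the grinder, tamping mat or coffee machine gets TAttachFilter enabled.
; Dropping disables all three and, if attached, turns off mesh physics.
; Overlapping a BP_ResetArea returns it to its spawn transform, and Using toggles grabbing through a component tag.
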(event `self.ReceiveBeginPlay`
  (set `self.Origin` (`self.GetTransform`)))

(event `self.Mesh.OnComponentBeginOverlap`
  (params (OverlappedComponent :type "PrimitiveComponent Object Reference") (OtherActor :type "Actor Object Reference") (OtherComp :type "PrimitiveComponent Object Reference") (OtherBodyIndex :type Integer) (bFromSweep :type Boolean) (SweepResult :type "HitResult Structure (by ref)"))
  (cast `/Game/CoreVR/Blueprints/Tools_Game/BP_ResetArea` OtherActor)
  (`PrimitiveComponent.SetSimulatePhysics` (`self.Mesh`) false)
  (`self.K2_SetActorTransform` (`self.Origin`))
  (`PrimitiveComponent.SetSimulatePhysics` (`self.Mesh`) true))

(event `Set State`
  (params (State :type "/Game/CoreVR/Blueprints/Tools_Maker/E_Porta Enum" :default "NewEnumerator0"))
  (bind _output_get (set `self.State` State))
  (switch `/Game/CoreVR/Blueprints/Tools_Maker/E_Porta` _output_get
    (:`NewEnumerator0`
      (`SceneComponent.SetVisibility` (`self.Tempered`) false false)
      (`SceneComponent.SetVisibility` (`self.UnTempered`) false false))
    (:`NewEnumerator1`
      (`SceneComponent.SetVisibility` (`self.Tempered`) false false)
      (`SceneComponent.SetVisibility` (`self.UnTempered`) true false))
    (:`NewEnumerator2`
      (`SceneComponent.SetVisibility` (`self.Tempered`) true false)
      (`SceneComponent.SetVisibility` (`self.UnTempered`) false false))))

(event `self.GrabComponent.OnDropped`
  (`|ExecutionSequence`
    (:`then_0`
      (if (`self.Attached?`)
        (`PrimitiveComponent.SetSimulatePhysics` (`self.Mesh`) false)
        (set `self.Attached?` false)))
    (:`then_1`
      (bind _returnvalue (`GameplayStatics.GetActorOfClass` "/Game/CoreVR/Blueprints/Tools_Maker/BP_CoffeeGrinder.BP_CoffeeGrinder_C"))
      (`/Game/CoreVR/Blueprints/Tools_Maker/BP_CoffeeGrinder.T_Attach_Filter` _returnvalue false))
    (:`then_2`
      (bind _returnvalue_2 (`GameplayStatics.GetActorOfClass` "/Game/CoreVR/Blueprints/Tools_Maker/BP_TempingMat.BP_TempingMat_C"))
      (`/Game/CoreVR/Blueprints/Tools_Maker/BP_TempingMat.T_Attach_Filter` _returnvalue_2 false))
    (:`then_3`
      (bind _returnvalue_3 (`GameplayStatics.GetActorOfClass` "/Game/CoreVR/Blueprints/Tools_Maker/BP_CoffeeMachine.BP_CoffeeMachine_C"))
      (`/Game/CoreVR/Blueprints/Tools_Maker/BP_CoffeeMachine.T_Attach_Filter` _returnvalue_3 false))))

(event `Using`
  (params (Using :type Boolean))
  (bind _componenttags (`ActorComponent.ComponentTags` (`self.GrabComponent`)))
  (if Using
    (`KismetArrayLibrary.Array_Set` _componenttags 0 "GrabDisable")
    (else
      (`KismetArrayLibrary.Array_Set` _componenttags))))

(event `self.GrabComponent.OnGrabbed`
  (switch `/Game/CoreVR/Blueprints/Tools_Maker/E_Porta` (`self.State`)
    (:`NewEnumerator0`
      (bind _returnvalue (`GameplayStatics.GetActorOfClass` "/Game/CoreVR/Blueprints/Tools_Maker/BP_CoffeeGrinder.BP_CoffeeGrinder_C"))
      (`/Game/CoreVR/Blueprints/Tools_Maker/BP_CoffeeGrinder.T_Attach_Filter` _returnvalue true))
    (:`NewEnumerator1`
      (bind _returnvalue_2 (`GameplayStatics.GetActorOfClass` "/Game/CoreVR/Blueprints/Tools_Maker/BP_TempingMat.BP_TempingMat_C"))
      (`/Game/CoreVR/Blueprints/Tools_Maker/BP_TempingMat.T_Attach_Filter` _returnvalue_2 true))
    (:`NewEnumerator2`
      (bind _returnvalue_3 (`GameplayStatics.GetActorOfClass` "/Game/CoreVR/Blueprints/Tools_Maker/BP_CoffeeMachine.BP_CoffeeMachine_C"))
      (`/Game/CoreVR/Blueprints/Tools_Maker/BP_CoffeeMachine.T_Attach_Filter` _returnvalue_3 true))))

(fn `UserConstructionScript`)