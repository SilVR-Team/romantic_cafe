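; VR coffee-making steamer machine that processes the contents of a milk cup.
; A cup overlapping the sphere snaps to the socket with sound and haptics, while text prompts toggle for attach, press and detach steps.
; A hand-tagged overlap on the button box starts a five-second cooldown with color, sound and haptic feedback.
; It moves one liquid type's amount into another in the cup, or shows steam if no cup is attached.
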(event `self.ReceiveTick`
  (params (DeltaSeconds :type "Float (single-precision)"))
  (bind _as_bp_milk_cup (`self.As BP Milk Cup`)
    (:`then`
      (if (> (`/Game/CoreVR/Blueprints/Tools_Liquid/BP_BaseCup.Now Amount` _as_bp_milk_cup) 0.0)
        (if (`self.Cooldown`)
          (`self.T_PressButton` false :!label _label)
          (else
            (switch `/Game/CoreVR/Blueprints/Tools_Liquid/E_Temp` (`/Game/CoreVR/Blueprints/Tools_Liquid/BP_BaseCup.Temp` _as_bp_milk_cup)
              (:`NewEnumerator5`
                (`self.T_PressButton` false))
              (:`NewEnumerator13`
                (`self.T_PressButton` true :!label _label_2))
              (:`NewEnumerator14`
                (goto _label_2)))))
        (else
          (goto _label))))
    (:`else`
      (`self.T_PressButton` false))))

(event `self.ReceiveBeginPlay`
  (bind _returnvalue (`PrimitiveComponent.CreateDynamicMaterialInstance` (`self.Cube1`) 0 "/Game/Asset/CustomMesh/Material/M_Button.M_Button" "None"))
  (set `self.MI_Button` _returnvalue)
  (`MaterialInstanceDynamic.SetVectorParameterValue` (`self.MI_Button`) "Color" (struct :`R` 1.0 :`A` 1.0)))

(event `self.Sphere.OnComponentBeginOverlap`
  (params (OverlappedComponent :type "PrimitiveComponent Object Reference") (OtherActor :type "Actor Object Reference") (OtherComp :type "PrimitiveComponent Object Reference") (OtherBodyIndex :type Integer) (bFromSweep :type Boolean) (SweepResult :type "HitResult Structure (by ref)"))
  (bind _asbp_milk_cup (cast `/Game/CoreVR/Blueprints/Tools_Liquid/BP_MilkCup` OtherActor))
  (bind _output_get (set `self.As BP Milk Cup` _asbp_milk_cup))
  (set `/Game/CoreVR/Blueprints/Tools_Liquid/BP_BaseCup.Attached?` true _output_get)
  (`SceneComponent.K2_AttachToComponent` (`/Game/CoreVR/Blueprints/Tools_Liquid/BP_BaseCup.Cup` _output_get) (`self.Socket_Porta`) "None" "SnapToTarget" "SnapToTarget" "KeepWorld" true)
  (`PlayerController.PlayHapticEffect` (`GameplayStatics.GetPlayerController` 0) "/Game/CoreVR/Haptics/AttachHapticEffect.AttachHapticEffect" (`/Game/CoreVR/Blueprints/Component/BP_GrabComponent.GetHeldByHand` (`/Game/CoreVR/Blueprints/Tools_Liquid/BP_BaseCup.GrabComponent` _output_get)) 0.5 false)
  (`GameplayStatics.PlaySoundAtLocation` "/Game/CoreVR/Audio/chulkuck_Cue.chulkuck_Cue" (`self.K2_GetActorLocation`) (struct) 1.0 1.0 0.0 null null null null)
  (`self.T_AttachMilk` false))

(event `self.Sphere.OnComponentEndOverlap`
  (params (OverlappedComponent :type "PrimitiveComponent Object Reference") (OtherActor :type "Actor Object Reference") (OtherComp :type "PrimitiveComponent Object Reference") (OtherBodyIndex :type Integer))
  (bind _as_bp_milk_cup (`self.As BP Milk Cup`))
  (if (== OtherActor _as_bp_milk_cup)
    (set `/Game/CoreVR/Blueprints/Tools_Liquid/BP_BaseCup.Attached?` false _as_bp_milk_cup)
    (set `self.As BP Milk Cup` null)
    (`self.T_Detach` false)))

(event `self.Box.OnComponentBeginOverlap`
  (params (OverlappedComponent :type "PrimitiveComponent Object Reference") (OtherActor :type "Actor Object Reference") (OtherComp :type "PrimitiveComponent Object Reference") (OtherBodyIndex :type Integer) (bFromSweep :type Boolean) (SweepResult :type "HitResult Structure (by ref)"))
  (bind _returnvalue (`GameplayStatics.GetPlayerController` 0))
  (if (not (`self.Cooldown`))
    (`self.T_PressButton` false)
    (set `self.Cooldown` true)
    (if (`ActorComponent.ComponentHasTag` OtherComp "Left")
      (`PlayerController.PlayHapticEffect` _returnvalue "/Game/CoreVR/Haptics/ButtonHapticEffect.ButtonHapticEffect" "Left" 0.5 false)
      (`MaterialInstanceDynamic.SetVectorParameterValue` (`self.MI_Button`) "Color" (struct :`R` 1.0 :`G` 1.0 :`B` 1.0 :`A` 1.0) :!label _label_3)
      (`GameplayStatics.PlaySoundAtLocation` "/Game/CoreVR/Audio/CoffeeMachine_ON_Cue.CoffeeMachine_ON_Cue" (`self.K2_GetActorLocation`) (struct) 1.0 1.0 0.0 null null null null)
      (bind _as_bp_milk_cup (`self.As BP Milk Cup`)
        (:`then`
          (`/Game/CoreVR/Blueprints/Tools_Liquid/BP_BaseCup.Using` _as_bp_milk_cup true)
          (`/Game/CoreVR/Blueprints/Tools_Liquid/BP_BaseCup.CloseMenu` _as_bp_milk_cup)
          (bind _now_liquid (`/Game/CoreVR/Blueprints/Tools_Liquid/BP_BaseCup.Now Liquid` _as_bp_milk_cup))
          (bind (_value _returnvalue_2) (`BlueprintMapLibrary.Map_Find` _now_liquid "NewEnumerator2"))
          (if _returnvalue_2
            (bind (_value_2 _returnvalue_3) (`BlueprintMapLibrary.Map_Find` _now_liquid "NewEnumerator1"))
            (if _returnvalue_3
              (`BlueprintMapLibrary.Map_Add` _now_liquid "NewEnumerator1" (+ _value _value_2))
              (else
                (`BlueprintMapLibrary.Map_Add` _now_liquid "NewEnumerator1" _value))))
          (`BlueprintMapLibrary.Map_Add` _now_liquid "NewEnumerator2")
          (`/Game/CoreVR/Blueprints/Tools_Liquid/BP_BaseCup.UpdateInfo` _as_bp_milk_cup))
        (:`else`
          (`SceneComponent.SetVisibility` (`self.Steam`) true false)))
      (`GameplayStatics.PlaySoundAtLocation` "/Game/CoreVR/Audio/Steamer_Cue.Steamer_Cue" (`self.K2_GetActorLocation`) (struct) 1.0 1.0 0.0 null null null null)
      (`KismetSystemLibrary.Delay` 5.0)
      (set `self.Cooldown` false)
      (bind _as_bp_milk_cup_2 (`self.As BP Milk Cup`)
        (:`then`
          (`/Game/CoreVR/Blueprints/Tools_Liquid/BP_BaseCup.Using` _as_bp_milk_cup_2 false))
        (:`else`
          _))
      (`MaterialInstanceDynamic.SetVectorParameterValue` (`self.MI_Button`) "Color" (struct :`R` 1.0 :`A` 1.0))
      (`SceneComponent.SetVisibility` (`self.Steam`) false false)
      (`GameplayStatics.PlaySoundAtLocation` "/Game/CoreVR/Audio/Steam_OFF_Cue.Steam_OFF_Cue" (`self.K2_GetActorLocation`) (struct) 1.0 1.0 0.0 null null null null)
      (`self.T_Detach` true)
      (elif (`ActorComponent.ComponentHasTag` OtherComp "Right")
        (`PlayerController.PlayHapticEffect` _returnvalue "/Game/CoreVR/Haptics/PistolFireHapticEffect.PistolFireHapticEffect" "Right" 0.5 false)
        (goto _label_3)
        (else
          (set `self.Cooldown` false))))))

(event `T_AttachMilk`
  (params (bNewVisibility :type Boolean))
  (`SceneComponent.SetVisibility` (`self.TextRender1`) bNewVisibility false))

(event `T_PressButton`
  (params (bNewVisibility :type Boolean))
  (`SceneComponent.SetVisibility` (`self.TextRender2`) bNewVisibility false))

(event `T_Detach`
  (params (bNewVisibility :type Boolean))
  (`SceneComponent.SetVisibility` (`self.TextRender3`) bNewVisibility false))

(fn `UserConstructionScript`)